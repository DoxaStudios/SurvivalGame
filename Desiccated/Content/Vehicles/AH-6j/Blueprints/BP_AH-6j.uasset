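; Player-controlled AH-6j helicopter with simple physics-based lift and direct rotation steering.
; The Helicopter Up axis adds velocity to Body along the actor's up vector, so tilting redirects thrust.
; Tick continuously spins the Engine component and applies local pitch and roll from combined move and mouse axes, with no yaw control.
; Box overlaps deal massive BP_Bullet_Damage to the sweep result's hit actor.
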(event OnComponentBeginOverlap(Box)
  (params (OverlappedComponent :type Primitive%20Component%20Object%20Reference) (OtherActor :type Actor%20Object%20Reference) (OtherComp :type Primitive%20Component%20Object%20Reference) (OtherBodyIndex :type Integer) (bFromSweep :type Boolean) (SweepResult :type Hit%20Result%20Structure%20%28by%20ref%29))
  (Game|Damage|ApplyDamage (.HitActor (Collision|BreakHitResult SweepResult)) 1e+05 0 0 "/Game/Damage_Types/BP_Bullet_Damage.BP_Bullet_Damage_C"))

(event EventTick
  (params (DeltaSeconds :type Float%20%28single-precision%29))
  (Variables|Util|SetDelta%20Seconds DeltaSeconds)
  (Utilities|FlowControl|Sequence
    (:then_0
      (Transformation|AddRelativeRotation (Variables|Default|GetEngine) (Math|Rotator|MakeRotator 0.0 0.0 (* (Variables|Util|GetDelta%20Seconds) 1e+03)) false false))
    (:then_1
      (Transformation|AddActorLocalRotation (Math|Rotator|MakeRotator (* (* (Variables|Util|GetDelta%20Seconds) 5e+01) (+ (Input|AxisValues|GetMoveRight) (Input|AxisValues|GetMouseX))) (* (* (Variables|Util|GetDelta%20Seconds) 5e+01) (+ (* (Input|AxisValues|GetMoveForward) -1.0) (* (Input|AxisValues|GetMouseY) -1.0))) 0.0) false false))))

(event Input|AxisEvents|InputAxisHelicopterUp
  (params (AxisValue :type Float%20%28single-precision%29))
  (Class|PrimitiveComponent|SetAllPhysicsLinearVelocity (Variables|Default|GetBody) (* (Math|Vector|GetUpVector (Transformation|GetActorRotation)) (* AxisValue 5e+01)) true))

(fn ConstructionScript)