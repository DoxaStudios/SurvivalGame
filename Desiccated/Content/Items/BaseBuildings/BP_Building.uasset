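; BP_Building is a building item that lets the player's BP_Huma character place props in the world.
; On BeginPlay, the authority spawns a BuildProp helper on the character's BuildLocation, configured with two buildables and upright, grid-snapped placement.
; Box overlap binds the character's fire and build-toggle inputs, with fire placing the prop.
; SetUse updates the build location, and the toggle handler switches building on alternate calls while in use.
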(event OnComponentEndOverlap(Placed)
  (params (OverlappedComponent :type Primitive%20Component%20Object%20Reference) (OtherActor :type Actor%20Object%20Reference) (OtherComp :type Primitive%20Component%20Object%20Reference) (OtherBodyIndex :type Integer))
  ;[1 1 1] Extra
  (Variables|Default|SetOverlap false))

(event OnComponentBeginOverlap(Box)
  (params (OverlappedComponent :type Primitive%20Component%20Object%20Reference) (OtherActor :type Actor%20Object%20Reference) (OtherComp :type Primitive%20Component%20Object%20Reference) (OtherBodyIndex :type Integer) (bFromSweep :type Boolean) (SweepResult :type Hit%20Result%20Structure%20%28by%20ref%29))
  (bind _building_ref (Variables|Default|GetBuilding%20ref))
  ;[1 1 1] Extra
  (Variables|Default|SetOverlap true)
  ;[1 1 1] calling binds
  (Utilities|FlowControl|Sequence
    (:then_0
      (EventDispatchers|BindEventtoFirePressed _building_ref (delegate Custom|FirePressed)))
    (:then_1
      (EventDispatchers|BindEventtoBuildTogg _building_ref (delegate Custom|togg)))))

(event Custom|Set%20Use
  (params (Use :type Boolean))
  (bind _building_ref (Variables|Default|GetBuilding%20ref))
  ;[1 1 1] Extra
  (Variables|Default|SetUse Use)
  (Default|SetBuildLocation (Variables|Default|GetBuild%20Prop) (Variables|/Game/Human/BP_Huma.BP_Huma_C|GetFPC _building_ref) (Variables|/Game/Human/BP_Huma.BP_Huma_C|GetBuildLocation_ _building_ref)))

(event Custom|FirePressed
  (CallFunction|Whateveriwant))

(event Custom|BuildTogg_Event
  (if (Variables|Default|GetUse)
    (if (Variables|Default|GetClicked)
      (Variables|Default|SetClicked false)
      (Default|ToggleBuilding (Variables|Default|GetBuild%20Prop))
      (else
        (Variables|Default|SetClicked true)))))

(event Custom|Whateveriwant
  (Default|PlaceProp (Variables|Default|GetBuild%20Prop)))

(event Custom|togg
  (CallFunction|BuildToggEvent))

(event EventBeginPlay
  (Utilities|FlowControl|Sequence
    (:then_0
      (bind _asbp_huma (Utilities|Casting|CastToBP_Huma (Game|GetPlayerCharacter 0)))
      (bind _output_get (Variables|Default|SetBuilding%20ref _asbp_huma))
      (if true
        (Networking|SwitchHasAuthority
          (:Authority
            (bind _returnvalue (Game|SpawnActorfromClass "/Game/Items/BaseBuildings/BuildCompoonents/BuildProp.BuildProp_C" (Math|Transform|MakeTransform "0, 0,0.000000" "0,0.000000,0.000000" "1,1.000000,1") "AlwaysSpawn" _output_get 0))
            (Class|Actor|AttachRootComponentto _returnvalue (Variables|/Game/Human/BP_Huma.BP_Huma_C|GetBuildLocation_ (Variables|Default|GetBuilding%20ref)) "None" "SnapToTarget" true)
            (bind _output_get_2 (Variables|Default|SetBuild%20Prop _returnvalue))
            ;[1 1 1] Custom
            (Default|Initialise _output_get_2 (Utilities|Array|MakeArray "/Game/Items/BaseBuildings/Ground_low.Ground_low" "/Engine/EditorMeshes/ArcadeEditorSphere.ArcadeEditorSphere") true 97.0 false 1.3e+02 true false 4e+02)))))))

(fn ConstructionScript
  (|CallParentFunction))

(fn True?
  (return (Variables|Default|GetTrue)))