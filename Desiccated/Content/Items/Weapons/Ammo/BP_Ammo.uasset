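; Ammo pickup Blueprint that adds one clip to the current weapon when its InteractE event fires.
; The increment goes through the Item reference's CurrentWeapon, behind a branch that is always true.
; Sphere overlap sets an Overlap flag and binds Interact_Event to the Interact dispatcher, but that handler is empty.
; The construction script only calls its parent.
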(event OnComponentBeginOverlap(Sphere)
  (params (OverlappedComponent :type Primitive%20Component%20Object%20Reference) (OtherActor :type Actor%20Object%20Reference) (OtherComp :type Primitive%20Component%20Object%20Reference) (OtherBodyIndex :type Integer) (bFromSweep :type Boolean) (SweepResult :type Hit%20Result%20Structure%20%28by%20ref%29))
  (Variables|Default|SetOverlap true)
  (Utilities|FlowControl|Sequence
    (:then_0
      (EventDispatchers|BindEventtoInteract (delegate Custom|Interact_Event)))))

(event Custom|InteractE
  (bind _item (Variables|Default|GetItem))
  (bind _currentweapon (Variables|/Game/Items/Item.Item_C|GetCurrentWeapon _item))
  (if true
    (Variables|/Game/Items/Weapons/Guns/BP_Gun.BP_Gun_C|SetClips _currentweapon (+ (Variables|/Game/Items/Weapons/Guns/BP_Gun.BP_Gun_C|GetClips _currentweapon) 1))))

(event Custom|Interact_Event)

(fn ConstructionScript
  (|CallParentFunction))