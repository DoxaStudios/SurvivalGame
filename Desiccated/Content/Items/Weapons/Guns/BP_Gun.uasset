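; BP_Gun is a data-driven gun actor that attaches to BP_Huma's weapon socket and handles firing, reloading and aim-down-sights.
; A WeaponStruct supplies ammo, animations, sounds and fire settings, and is rebuilt whenever rounds change.
; Single shots spawn a projectile or run a spread debug line trace without hit handling, then play montages and spend rounds.
; Rapid fire uses a looping timer that only spawns projectiles, skipping ammo and effects.
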(event Custom|Equip
  (bind _asbp_huma (Utilities|Casting|CastToBP_Huma (Components|GetOwner)))
  (Class|SceneComponent|Attachto (Variables|Default|GetGun%20Mesh) (Variables|/Script/Engine.Character|GetMesh _asbp_huma) "WeaponSocket" "SnapToTarget" true)
  (Variables|Default|SetEquiped true)
  (Rendering|SetActorHiddenInGame false))

(event Custom|Reload%20Animation%20On%20All
  (bind _weapon_struct (Variables|Default|GetWeapon%20Struct))
  (bind _normalanims (Utilities|Struct|BreakWeaponStruct _weapon_struct))
  (Animation|Montage|MontagePlay (Components|SkeletalMesh|GetAnimInstance (Variables|/Script/Engine.Character|GetMesh (Variables|Default|GetCharacter))) (Utilities|Array|Get(acopy) _normalanims 2) 1.0)
  (Animation|Montage|MontagePlay (Variables|Default|GetAnim%20Instance) (Utilities|Array|Get(acopy) _normalanims 3) 1.0))

(event Custom|Run%20on%20other
  (bind _character (Variables|Default|GetCharacter))
  (Animation|Montage|MontageIsPlaying (Components|SkeletalMesh|GetAnimInstance (Variables|Default|GetGun%20Mesh)) 0)
  (if (Math|Boolean|ANDBoolean (not (Variables|/Game/Human/BP_Huma.BP_Huma_C|GetSprinting _character)) (not (Variables|/Game/Human/BP_Huma.BP_Huma_C|GetADS _character)) (> (.Clips (Utilities|Struct|BreakWeaponStruct (Variables|Default|GetWeapon%20Struct))) 0) (!= (.Rounds (Utilities|Struct|BreakWeaponStruct (Variables|Default|GetWeapon%20Struct))) (.ClipsSize (Utilities|Struct|BreakWeaponStruct (Variables|Default|GetWeapon%20Struct)))))
    (CallFunction|ReloadAnimationonAll)
    (Utilities|FlowControl|Delay 0.5)
    (Variables|Default|SetWeapon%20Struct (Utilities|Struct|MakeWeaponStruct (- (.Clips (Utilities|Struct|BreakWeaponStruct (Variables|Default|GetWeapon%20Struct))) 1) (.ClipsSize (Utilities|Struct|BreakWeaponStruct (Variables|Default|GetWeapon%20Struct))) (.ClipsSize (Utilities|Struct|BreakWeaponStruct (Variables|Default|GetWeapon%20Struct))) (.Projectile (Utilities|Struct|BreakWeaponStruct (Variables|Default|GetWeapon%20Struct))) (.FiringSound (Utilities|Struct|BreakWeaponStruct (Variables|Default|GetWeapon%20Struct))) (.ReloadSound (Utilities|Struct|BreakWeaponStruct (Variables|Default|GetWeapon%20Struct))) (.EmptyClipSound (Utilities|Struct|BreakWeaponStruct (Variables|Default|GetWeapon%20Struct))) (.ADSAnims (Utilities|Struct|BreakWeaponStruct (Variables|Default|GetWeapon%20Struct))) (.NormalAnims (Utilities|Struct|BreakWeaponStruct (Variables|Default|GetWeapon%20Struct))) (.WeaponType (Utilities|Struct|BreakWeaponStruct (Variables|Default|GetWeapon%20Struct))) (.ShotType (Utilities|Struct|BreakWeaponStruct (Variables|Default|GetWeapon%20Struct))) (.TimeBetweenShot (Utilities|Struct|BreakWeaponStruct (Variables|Default|GetWeapon%20Struct))) (.ShotCount (Utilities|Struct|BreakWeaponStruct (Variables|Default|GetWeapon%20Struct))) (.SpreadX (Utilities|Struct|BreakWeaponStruct (Variables|Default|GetWeapon%20Struct))) (.SpreadY (Utilities|Struct|BreakWeaponStruct (Variables|Default|GetWeapon%20Struct))) (.Range (Utilities|Struct|BreakWeaponStruct (Variables|Default|GetWeapon%20Struct))) (.MuzzleFlash (Utilities|Struct|BreakWeaponStruct (Variables|Default|GetWeapon%20Struct)))))
    (Audio|PlaySoundatLocation 0 (Transformation|GetWorldLocation (Variables|Default|GetGun%20Mesh)))
    (Development|PrintString "Hello")))

(event Custom|Set%20Weapon%20Struct
  (params (Weapon%20Struct :type Weapon%20Struct%20Structure))
  (Variables|Default|SetWeapon%20Struct Weapon%20Struct))

(event Custom|Unequip
  (Utilities|Casting|CastToBP_Huma (Components|GetOwner))
  (Class|SceneComponent|DetachfromParent (Variables|Default|GetGun%20Mesh) false true)
  (Rendering|SetActorHiddenInGame true)
  (Variables|Default|SetEquiped false))

(event Custom|Reload
  (CallFunction|RunonOther))

(event Custom|ADS
  (params (Released :type Boolean))
  (bind _character (Variables|Default|GetCharacter))
  (if (not Released)
    (if (not (Variables|/Game/Human/BP_Huma.BP_Huma_C|GetSprinting _character))
      (Default|SetADS _character true))
    (else
      (Default|SetADS _character false))))

(event Custom|Fire%20Weapon
  (params (Released :type Boolean))
  (bind _weapon_struct (Variables|Default|GetWeapon%20Struct))
  (bind _weapon_struct_2 (Variables|Default|GetWeapon%20Struct))
  (bind (_clips _rounds _clipssize _projectile _firingsound _reloadsound _emptyclipsound _adsanims _normalanims) (Utilities|Struct|BreakWeaponStruct _weapon_struct))
  (bind (_clips_2 _rounds_2 _clipssize_2 _projectile_2 _firingsound_2 _reloadsound_2 _emptyclipsound_2 _adsanims_2 _normalanims_2 _weapontype) (Utilities|Struct|BreakWeaponStruct _weapon_struct_2))
  (bind _returnvalue (> _rounds 0))
  (if (not Released)
    (bind _returnvalue_2 (Animation|Montage|MontageIsPlaying (Variables|Default|GetAnim%20Instance) (Utilities|Array|Get(acopy) _normalanims 3)))
    (if (Math|Boolean|ANDBoolean (not (Variables|/Game/Human/BP_Huma.BP_Huma_C|GetSprinting (Variables|Default|GetCharacter))) _returnvalue (not _returnvalue_2))
      (switch Utilities|FlowControl|Switch|SwitchonWeaponType _weapontype
        (:NewEnumerator0
          (CallFunction|SingleShot))
        (:NewEnumerator1
          (bind _returnvalue_3 (Utilities|Time|SetTimerbyFunctionName self "RapidFire" (.TimeBetweenShot (Utilities|Struct|BreakWeaponStruct (Variables|Default|GetWeapon%20Struct))) true))
          (Variables|Default|SetTimerHand _returnvalue_3)))
      (elif _returnvalue
        (Audio|PlaySoundatLocation _emptyclipsound_2 (Transformation|GetWorldLocation (Variables|Default|GetGun%20Mesh)))))
    (else
      (Utilities|Time|ClearandInvalidateTimerbyHandle (Variables|Default|GetTimerHand)))))

(event EventTick
  (params (DeltaSeconds :type Float%20%28single-precision%29))
  (bind _weapon_struct (Variables|Default|GetWeapon%20Struct))
  (bind (_clips _rounds _clipssize _projectile _firingsound _reloadsound _emptyclipsound _adsanims _normalanims _weapontype _shottype _timebetweenshot _shotcount _spreadx _spready _range _muzzleflash) (Utilities|Struct|BreakWeaponStruct _weapon_struct))
  (bind _output_get (Variables|Default|SetClips (+ _clips (Variables|Default|GetClips))))
  (if (> _rounds _clipssize)
    (CallFunction|SetWeaponStruct (Utilities|Struct|MakeWeaponStruct _output_get _clipssize _clipssize _projectile _firingsound _reloadsound _emptyclipsound _adsanims _normalanims _weapontype _shottype _timebetweenshot _shotcount _spreadx _spready _range _muzzleflash))))

(fn ConstructionScript
  (|CallParentFunction)
  (Variables|Default|SetAnim%20Instance (Components|SkeletalMesh|GetAnimInstance (Variables|Default|GetGun%20Mesh))))

(fn LineTraceShot
  (bind _gun_mesh (Variables|Default|GetGun%20Mesh))
  (bind _weapon_struct (Variables|Default|GetWeapon%20Struct))
  (bind _weapon_struct_2 (Variables|Default|GetWeapon%20Struct))
  (bind _weapon_struct_3 (Variables|Default|GetWeapon%20Struct))
  (bind _character (Variables|Default|GetCharacter))
  (bind _character_2 (Variables|Default|GetCharacter))
  (bind (_clips _rounds _clipssize _projectile _firingsound _reloadsound _emptyclipsound _adsanims _normalanims _weapontype _shottype _timebetweenshot _shotcount _spreadx _spready) (Utilities|Struct|BreakWeaponStruct _weapon_struct))
  (bind (_clips_2 _rounds_2 _clipssize_2 _projectile_2 _firingsound_2 _reloadsound_2 _emptyclipsound_2 _adsanims_2 _normalanims_2) (Utilities|Struct|BreakWeaponStruct _weapon_struct_2))
  (bind (_clips_3 _rounds_3 _clipssize_3 _projectile_3 _firingsound_3 _reloadsound_3 _emptyclipsound_3 _adsanims_3 _normalanims_3 _weapontype_2 _shottype_2 _timebetweenshot_2 _shotcount_2 _spreadx_2 _spready_2 _range _muzzleflash) (Utilities|Struct|BreakWeaponStruct _weapon_struct_3))
  (bind _returnvalue (Transformation|GetSocketLocation _gun_mesh "Muzzle"))
  (bind _mesh (Variables|/Script/Engine.Character|GetMesh _character_2))
  (bind _capsulecomponent (Variables|/Script/Engine.Character|GetCapsuleComponent _character))
  (bind _returnvalue_2 (Math|Vector|GetForwardVector _capsulecomponent))
  (bind (_x _y _z) (Math|Vector|BreakVector _returnvalue_2))
  (Development|PrintString "Hello")
  (Collision|LineTraceByChannel _returnvalue (+ _returnvalue (* (Math|Vector|MakeVector (+ _x (Math|Random|RandomFloatinRange (* _spreadx -1.0) _spreadx)) (+ _y (Math|Random|RandomFloatinRange (* _spready -1.0) _spready)) _z) (.Range (Utilities|Struct|BreakWeaponStruct (Variables|Default|GetWeapon%20Struct))))) "TraceTypeQuery1" false 0 "Persistent")
  (if (Variables|/Game/Human/BP_Huma.BP_Huma_C|GetADS _character_2)
    (Animation|Montage|MontagePlay (Components|SkeletalMesh|GetAnimInstance _mesh) (Utilities|Array|Get(acopy) _adsanims_2) 1.0)
    (Animation|Montage|MontagePlay (Variables|Default|GetAnim%20Instance) (Utilities|Array|Get(acopy) _adsanims_2 1) 1.0)
    (else
      (Animation|Montage|MontagePlay (Components|SkeletalMesh|GetAnimInstance _mesh) (Utilities|Array|Get(acopy) _normalanims_2) 1.0)
      (Animation|Montage|MontagePlay (Variables|Default|GetAnim%20Instance) (Utilities|Array|Get(acopy) _normalanims_2 1) 1.0)))
  (CallFunction|SetWeaponStruct (Utilities|Struct|MakeWeaponStruct _clips_3 (- _rounds_3 _shotcount_2) _clipssize_3 _projectile_3 _firingsound_3 _reloadsound_3 _emptyclipsound_3 _adsanims_3 _normalanims_3 _weapontype_2 _shottype_2 _timebetweenshot_2 _shotcount_2 _spreadx_2 _spready_2 _range _muzzleflash))
  (Audio|PlaySoundatLocation (.FiringSound (Utilities|Struct|BreakWeaponStruct (Variables|Default|GetWeapon%20Struct))) (Transformation|GetSocketLocation (Variables|Default|GetGun%20Mesh) "Muzzle")))

(fn ProjectileShot
  (bind _weapon_struct (Variables|Default|GetWeapon%20Struct))
  (bind _weapon_struct_2 (Variables|Default|GetWeapon%20Struct))
  (bind _character (Variables|Default|GetCharacter))
  (bind (_clips _rounds _clipssize _projectile _firingsound _reloadsound _emptyclipsound _adsanims _normalanims _weapontype _shottype _timebetweenshot _shotcount _spreadx _spready _range _muzzleflash) (Utilities|Struct|BreakWeaponStruct _weapon_struct))
  (bind (_clips_2 _rounds_2 _clipssize_2 _projectile_2 _firingsound_2 _reloadsound_2 _emptyclipsound_2 _adsanims_2 _normalanims_2) (Utilities|Struct|BreakWeaponStruct _weapon_struct_2))
  (bind _mesh (Variables|/Script/Engine.Character|GetMesh _character))
  (bind _returnvalue (Game|SpawnActorfromClass (.Projectile (Utilities|Struct|BreakWeaponStruct (Variables|Default|GetWeapon%20Struct))) (Math|Transform|MakeTransform (Transformation|GetSocketLocation (Variables|Default|GetGun%20Mesh) "Muzzle") (Transformation|GetWorldRotation (Variables|/Script/Engine.Character|GetCapsuleComponent (Variables|Default|GetCharacter)))) "Undefined" 0 0))
  (Actor|SetOwner _returnvalue 0)
  (if (Variables|/Game/Human/BP_Huma.BP_Huma_C|GetADS _character)
    (Animation|Montage|MontagePlay (Components|SkeletalMesh|GetAnimInstance _mesh) (Utilities|Array|Get(acopy) _adsanims_2) 1.0)
    (Animation|Montage|MontagePlay (Variables|Default|GetAnim%20Instance) (Utilities|Array|Get(acopy) _adsanims_2 1) 1.0)
    (else
      (Animation|Montage|MontagePlay (Components|SkeletalMesh|GetAnimInstance _mesh) (Utilities|Array|Get(acopy) _normalanims_2) 1.0)
      (Animation|Montage|MontagePlay (Variables|Default|GetAnim%20Instance) (Utilities|Array|Get(acopy) _normalanims_2 1) 1.0)))
  (CallFunction|SetWeaponStruct (Utilities|Struct|MakeWeaponStruct _clips (- _rounds _shotcount) _clipssize _projectile _firingsound _reloadsound _emptyclipsound _adsanims _normalanims _weapontype _shottype _timebetweenshot _shotcount _spreadx _spready _range _muzzleflash))
  (Audio|PlaySoundatLocation (.FiringSound (Utilities|Struct|BreakWeaponStruct (Variables|Default|GetWeapon%20Struct))) (Transformation|GetSocketLocation (Variables|Default|GetGun%20Mesh) "Muzzle")))

(fn SingleShot
  (switch Utilities|FlowControl|Switch|SwitchonShotType (.ShotType (Utilities|Struct|BreakWeaponStruct (Variables|Default|GetWeapon%20Struct)))
    (:NewEnumerator0
      (CallFunction|ProjectileShot))
    (:NewEnumerator1
      (CallFunction|LineTraceShot))))

(fn BreakStruct
  (params (WeaponStruct :type Weapon%20Struct%20Structure%20%28by%20ref%29))
  (bind (_clips _rounds _clipssize _projectile _firingsound _reloadsound _emptyclipsound _adsanims _normalanims _weapontype _shottype _timebetweenshot _shotcount _spreadx _spready _range _muzzleflash) (Utilities|Struct|BreakWeaponStruct WeaponStruct))
  (return _clips _rounds _clipssize _projectile _firingsound _reloadsound _emptyclipsound _adsanims _normalanims _weapontype _shottype _timebetweenshot _shotcount _spreadx _spready _range _muzzleflash))

(fn MakeStruct
  (params (Clips :type Integer) (Rounds :type Integer) (ClipsSize :type Integer) (Projectile :type Actor%20Class%20Reference) (FiringSound :type Sound%20Cue%20Object%20Reference) (ReloadSound :type Sound%20Cue%20Object%20Reference) (EmptyClipSound :type Sound%20Cue%20Object%20Reference) (ADSAnims :type Array%20of%20Anim%20Montage%20Object%20References) (NormalAnims :type Array%20of%20Anim%20Montage%20Object%20References) (WeaponType :type WeaponType%20Enum) (ShotType :type ShotType%20Enum) (TimeBetweenShot :type Float%20%28single-precision%29) (ShotCount :type Integer) (SpreadX :type Float%20%28single-precision%29) (SpreadY :type Float%20%28single-precision%29) (Range :type Float%20%28single-precision%29) (MuzzleFlash :type Array%20of%20Particle%20System%20Object%20References)))

(fn Rapidfire
  (if (Variables|/Game/Human/BP_Huma.BP_Huma_C|GetFireDown (Variables|Default|GetCharacter))
    (Game|SpawnActorfromClass (.Projectile (Utilities|Struct|BreakWeaponStruct (Variables|Default|GetWeapon%20Struct))) (Math|Transform|MakeTransform (Transformation|GetSocketLocation (Variables|Default|GetGun%20Mesh) "Muzzle") (Transformation|GetWorldRotation (Variables|/Script/Engine.Character|GetCapsuleComponent (Variables|Default|GetCharacter)))) "Undefined" 0 0)))