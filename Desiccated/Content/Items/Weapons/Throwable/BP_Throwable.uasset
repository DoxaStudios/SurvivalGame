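; Throwable explosive weapon that a BP_Huma owner throws from its inventory and that detonates after a short fuse.
; Action 0 triggers the throw through Explosion and ReplicateToAll, then clears the item's inventory slot.
; The throw teleports the mesh in front of the owner's aim, unhides it and applies velocity-based and radial force impulses.
; After the delay it plays explosion effects, deals falloff radial damage and destroys itself.
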(event Custom|Explosion
  (CallFunction|ReplicatetoAll))

(event Custom|Effects
  (bind _mesh (Variables|Character|GetMesh))
  (bind _returnvalue (Transformation|GetWorldLocation _mesh))
  (Effects|SpawnEmitteratLocation "/Game/Imports/StarterContent/Particles/P_Explosion.P_Explosion" _returnvalue "0, 0,0.000000")
  (Audio|PlaySoundatLocation "/Game/Items/Weapons/Throwable/PipeBomb/Sound/S_PipeBomb_Explosion_1.S_PipeBomb_Explosion_1" _returnvalue "0, 0, 0" 1.0 1.0 0.0 "/Game/DriveablePack/Audio/Engine/Engine_att.Engine_att"))

(event Custom|Replicate%20to%20all
  (bind _asbp_huma (Utilities|Casting|CastToBP_Huma (Components|GetOwner)))
  (Transformation|SetWorldTransform (Variables|Character|GetMesh) (Math|Transform|MakeTransform (+ (Transformation|GetActorLocation _asbp_huma) (Math|Vector|RotateVector "50.000000,25.000000,100.000000" (Pawn|GetControlRotation _asbp_huma :!class /Script/Engine.Pawn))) "0, 0, 0" "1,1.000000,1") false true)
  (Rendering|SetActorHiddenInGame false)
  (Collision|SetActorEnableCollision true)
  (Physics|AddImpulseatLocation (Variables|Character|GetMesh) (* (Transformation|GetVelocity) "1.000000,1.000000,1.000000") (Transformation|GetActorLocation) "None")
  (Class|RadialForceComponent|FireImpulse (Variables|Default|GetRadialForce))
  (Utilities|FlowControl|Delay 3.0)
  (CallFunction|Effects)
  (bind _returnvalue (Class|GameplayStatics|ApplyRadialDamagewithFalloff 1e+02 1e+01 (Transformation|GetWorldLocation (Variables|Character|GetMesh)) 1e+02 2e+02 5.0 "/Game/Damage_Types/BP_Bullet_Damage.BP_Bullet_Damage_C" 0 self 0 "ECC_Visibility"))
  (if _returnvalue
    _
    (else
      _))
  (Actor|DestroyActor))

(event EventAction
  (params (Action :type Integer))
  (switch int Action
    (:0
      (CallFunction|Explosion)
      (bind _asbp_huma (Utilities|Casting|CastToBP_Huma (Components|GetOwner)))
      (Utilities|Array|SetArrayElem (Variables|/Game/Human/BP_Huma.BP_Huma_C|GetInventory _asbp_huma) (Utilities|Array|FindItem (Variables|/Game/Human/BP_Huma.BP_Huma_C|GetInventory _asbp_huma) self) 0))))

(fn ConstructionScript)