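; Parent helicopter Blueprint for the AH-6j vehicle folder, handling physics lift, tilt, blade spin and contact damage.
; The up axis accumulates a clamped hover velocity, added to Body's physics velocity along the actor's up vector.
; On Tick, remote instances pass move and mouse axes through SendInput, while authority spins Engine and applies stored input as pitch and roll.
; Box overlaps apply massive bullet-type damage to the sweep's hit actor.
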(event OnComponentBeginOverlap(Box)
  (params (OverlappedComponent :type Primitive%20Component%20Object%20Reference) (OtherActor :type Actor%20Object%20Reference) (OtherComp :type Primitive%20Component%20Object%20Reference) (OtherBodyIndex :type Integer) (bFromSweep :type Boolean) (SweepResult :type Hit%20Result%20Structure%20%28by%20ref%29))
  (Game|Damage|ApplyDamage (.HitActor (Collision|BreakHitResult SweepResult)) 1e+05 0 0 "/Game/Damage_Types/BP_Bullet_Damage.BP_Bullet_Damage_C"))

(event Custom|Send%20Input
  (params (Forward%20Input :type Vector%202D%20Structure) (Right%20Input :type Vector%202D%20Structure))
  (Variables|Input|SetForward%20Input Forward%20Input)
  (Variables|Input|SetRight%20Input Right%20Input))

(event Custom|Up%20Movement
  (params (Input :type Vector))
  (Class|PrimitiveComponent|SetAllPhysicsLinearVelocity (Variables|Default|GetBody) Input true))

(event Custom|Rotate%20Blade%20On%20All
  (Transformation|AddRelativeRotation (Variables|Default|GetEngine) (Math|Rotator|MakeRotator 0.0 0.0 (* (Variables|Util|GetDelta%20Seconds) 1e+03)) false false))

(event Custom|Set%20Hover%20Velocity
  (params (Input :type Float%20%28single-precision%29))
  (Variables|Util|SetHover%20Velocity Input))

(event EventTick
  (params (DeltaSeconds :type Float%20%28single-precision%29))
  (bind _forward_input (Variables|Input|GetForward%20Input))
  (bind _right_input (Variables|Input|GetRight%20Input))
  (bind (_x _y) (Math|Vector2D|BreakVector2D _forward_input))
  (bind (_x_2 _y_2) (Math|Vector2D|BreakVector2D _right_input))
  (Variables|Util|SetDelta%20Seconds DeltaSeconds)
  (Networking|SwitchHasAuthority
    (:Authority
      (Utilities|FlowControl|Sequence
        (:then_0
          (CallFunction|RotateBladeonAll))
        (:then_1
          (Transformation|AddActorLocalRotation (Math|Rotator|MakeRotator (* (* (Variables|Util|GetDelta%20Seconds) 5e+01) (+ _x_2 _y_2)) (* (* (Variables|Util|GetDelta%20Seconds) 5e+01) (+ (* _x -1.0) (* _y -1.0))) 0.0) false false))))
    (:Remote
      (CallFunction|SendInput (Math|Vector2D|MakeVector2D (Input|AxisValues|GetMoveForward) (Input|AxisValues|GetMouseY)) (Math|Vector2D|MakeVector2D (Input|AxisValues|GetMoveRight) (Input|AxisValues|GetMouseX))))))

(event Input|AxisEvents|InputAxisHelicopterUp
  (params (AxisValue :type Float%20%28single-precision%29))
  (bind _returnvalue (!= AxisValue 0.0))
  (bind _returnvalue_2 (* AxisValue 1.0))
  (bind _hover_velocity (Variables|Default|Gethover%20velocity))
  (bind _returnvalue_3 (Math|Float|SelectFloat _returnvalue_2 0.0 _returnvalue))
  (bind _returnvalue_4 (+ _returnvalue_3 _hover_velocity))
  (bind _returnvalue_5 (Math|Float|Clamp(Float) _returnvalue_4 -7e+01 7e+01))
  (if _returnvalue
    (CallFunction|SetHoverVelocity _returnvalue_5)
    (CallFunction|UpMovement (* (Math|Vector|GetUpVector (Transformation|GetActorRotation)) _returnvalue_5))
    (else
      (Math|Float|CompareFloat (Variables|Default|Gethover%20velocity) 0.0
        (:>
          (CallFunction|SetHoverVelocity 11.0 :!label _label))
        (:==
          (CallFunction|SetHoverVelocity 0.0))
        (:<
          (goto _label))))))

(fn ConstructionScript)

(fn OnRepHoverVelocity)