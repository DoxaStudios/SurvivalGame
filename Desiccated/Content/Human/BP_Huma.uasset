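; Player human character with first/third-person views, stance-based movement speeds, ADS and clamped free look that eases back on release.
; A server interact trace stores Items in an inventory array or possesses vehicles and hover bikes.
; Input routes fire and reload to the selected hotbar item, while Tick equips it and unequips the others.
; Health is rudimentary: damage only prints a computed value without storing it, and Tick triggers death at zero.
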(event Custom|Set%20Combat%20Mode
  (params (Combat%20Mode :type Boolean))
  ;[1 1 1] Set Combat Mode
  (Variables|CharacterInfo|SetCombatMode Combat%20Mode))

(event Custom|Set%20ADS
  (params (ADS :type Boolean))
  ;[1 1 1] Ads
  (Variables|CharacterInfo|SetADS ADS))

(event Custom|Interact%28Server%29
  (bind _returnvalue (Pawn|GetController))
  (bind _tpc (Variables|Default|GetTPC))
  (bind _returnvalue_2 (Transformation|GetWorldLocation _tpc))
  ;[1 1 1] Interact
  (bind _outhit (Collision|LineTraceByChannel _returnvalue_2 (+ _returnvalue_2 (* (Math|Vector|GetForwardVector _tpc) (+ (Variables|/Script/Engine.SpringArmComponent|GetTargetArmLength (Variables|Default|GetSpringArm)) (Variables|Util|GetInteract%20Distance)))) "TraceTypeQuery1" false 0 "Persistent"))
  (if (Utilities|ClassIsChildOf (Utilities|GetClass (.HitActor (Collision|BreakHitResult _outhit))) "/Game/Items/Item.Item_C")
    (bind _asitem (Utilities|Casting|CastToItem (.HitActor (Collision|BreakHitResult _outhit))))
    (bind _index (CallFunction|GetSpacetoAddItem))
    (if (!= _index -1)
      (Utilities|Array|SetArrayElem (Variables|Inventory|GetInventory) _index _asitem)
      (Default|Pickup _asitem self)
      (if (Utilities|ClassIsChildOf (Utilities|GetClass _asitem) "/Game/Items/Weapons/Guns/BP_Gun.BP_Gun_C")
        (bind _asbp_gun (Utilities|Casting|CastToBP_Gun _asitem))
        (bind _output_get (Variables|/Game/Items/Weapons/Guns/BP_Gun.BP_Gun_C|SetCharacter _asbp_gun self))
        (Actor|SetOwner _asbp_gun _output_get)))
    (elif (Utilities|ClassIsChildOf (Utilities|GetClass (.HitActor (Collision|BreakHitResult _outhit))) "/Script/Engine.WheeledVehicle")
      (bind _aswheeled_vehicle (Utilities|Casting|CastToWheeledVehicle (.HitActor (Collision|BreakHitResult _outhit))))
      (Pawn|Possess _returnvalue _aswheeled_vehicle)
      (elif (Utilities|ClassIsChildOf (Utilities|GetClass (.HitActor (Collision|BreakHitResult _outhit))) "/Game/Vehicles/HoverBike/HoverBikeP.HoverBikeP_C")
        (bind _ashover_bike_p (Utilities|Casting|CastToHoverBikeP (.HitActor (Collision|BreakHitResult _outhit))))
        (Pawn|Possess _returnvalue _ashover_bike_p)))))

(event Custom|Server%20Switch%20View
  (params (First%20Person :type Boolean))
  ;[1 1 1] Toggle Camera View
)

(event Custom|Move%20Item
  (params (Old :type Integer) (New :type Integer))
  ;[1 1 1] Move Item
  (CallFunction|SwitchInventoryItem Old New))

(event Custom|Set%20Hotbar%20Index
  (params (Index :type Integer))
  ;[1 1 1] Set Hotbar Index on server
  (if (== Index -1)
    (Variables|Inventory|SetHotBarIndex 6)
    (elif (== Index 7)
      (Variables|Inventory|SetHotBarIndex 0)
      (else
        (Variables|Inventory|SetHotBarIndex Index)))))

(event Custom|Spawn%20Actor%20On%20Server
  (params (Actor :type Actor%20Class%20Reference) (Transform :type Transform))
  ;[1 1 1] Spawn Actor on Server
  (Game|SpawnActorfromClass Actor Transform "Undefined" 0 0))

(event Custom|Print%20to%20Client
  (params (Input :type String))
  ;[1 1 1] Print to Client
  (Development|PrintString Input))

(event Custom|Fire%20Trace
  (bind _tpc (Variables|Default|GetTPC))
  (bind _returnvalue (Transformation|GetWorldLocation _tpc))
  ;[1 1 1] Fire Trace
  (bind (_outhit _returnvalue_2) (Collision|LineTraceByChannel _returnvalue (+ _returnvalue (* (Math|Vector|GetForwardVector _tpc) (+ (Variables|/Script/Engine.SpringArmComponent|GetTargetArmLength (Variables|Default|GetSpringArm)) (Variables|Util|GetHand%20Interact%20Distance)))) "TraceTypeQuery1" false 0 "Persistent" true "(R=0.000000,G=0.000000,B=0.000000,A=1.000000)" "(R=0.000000,G=0.000000,B=0.000000,A=1.000000)"))
  (if _returnvalue_2
    _))

(event Custom|Set%20Sprinting
  (params (Sprinting :type Boolean))
  ;[0 1 1] Movement
  (Variables|CharacterInfo|SetSprinting Sprinting))

(event Custom|Set%20Movement%20Speed
  (params (Speed :type Float%20%28single-precision%29))
  ;[0 1 1] Movement
  (Variables|/Script/Engine.CharacterMovementComponent|SetMaxWalkSpeed (Variables|Character|GetCharacterMovement) Speed))

(event Custom|Change%20Stance
  (params (Stance :type EN_Stance_Type%20Enum))
  ;[1 1 1] Change Stance
  (switch Utilities|FlowControl|Switch|SwitchonEN_Stance_Type Stance
    (:NewEnumerator0
      (switch Utilities|FlowControl|Switch|SwitchonEN_Stance_Type (Variables|CharacterInfo|GetStance)
        (:NewEnumerator0
          _)
        (:NewEnumerator1
          _)
        (:NewEnumerator2
          _)
        (:NewEnumerator3
          _)))
    (:NewEnumerator1
      _)
    (:NewEnumerator2
      (switch Utilities|FlowControl|Switch|SwitchonEN_Stance_Type (Variables|CharacterInfo|GetStance)
        (:NewEnumerator0
          (Animation|Montage|MontagePlay (Components|SkeletalMesh|GetAnimInstance (Variables|Character|GetMesh)) 0 1.0))
        (:NewEnumerator1
          _)
        (:NewEnumerator2
          _)
        (:NewEnumerator3
          _))))
  (Variables|CharacterInfo|SetStance Stance))

(event Game|Damage|EventAnyDamage
  (params (Damage :type Float%20%28single-precision%29) (DamageType :type Damage%20Type%20Object%20Reference) (InstigatedBy :type Controller%20Object%20Reference) (DamageCauser :type Actor%20Object%20Reference))
  ;[1 1 1] Any Damage
  (bind _health (CallFunction|Health self Damage))
  (Development|PrintString (Utilities|String|ToString(Float) _health)))

(event EventBeginPlay
  (bind _returnvalue (Game|GetPlayerCameraManager 0))
  (bind _textrender (Variables|Default|GetTextRender))
  ;[1 1 1] Beign Play
  (Utilities|FlowControl|Sequence
    (:then_0
      (Variables|/Script/Engine.PlayerCameraManager|SetViewPitchMax _returnvalue 8e+01)
      (Variables|/Script/Engine.PlayerCameraManager|SetViewPitchMin _returnvalue -7e+01))
    (:then_2
      (Networking|SwitchHasAuthority
        (:Authority
          (Rendering|Components|TextRender|SetText _textrender (Utilities|Text|ToText(String) (Class|AdvancedSessionsLibrary|GetPlayerName (Game|GetPlayerController 0)))))
        (:Remote
          (Rendering|Components|TextRender|SetText _textrender (Utilities|Text|ToText(String) (Utilities|String|BuildString(Float) "" "Health:" (Variables|CharacterInfo|GetHealth)))))))))

(event EventTick
  (params (DeltaSeconds :type Float%20%28single-precision%29))
  (bind _returnvalue (Pawn|GetControlRotation :!class /Script/Engine.Pawn))
  (bind _freelooksavedrotation (Variables|Util|GetFreeLookSavedRotation))
  (bind _inventory (Variables|Inventory|GetInventory))
  (bind _hotbarindex (Variables|Inventory|GetHotBarIndex))
  (bind _item (Utilities|Array|Get(acopy) _inventory _hotbarindex))
  (bind _yaw (Math|Rotator|BreakRotator _returnvalue))
  (bind _returnvalue_2 (Utilities|GetClass _item))
  (bind _returnvalue_3 (- _yaw _freelooksavedrotation))
  ;[1 1 1] Tick
  (Utilities|FlowControl|Sequence
    (:then_0
      (if (<= (Variables|CharacterInfo|GetHealth) 0.0)
        (Physics|SetSimulatePhysics (Variables|Character|GetMesh) true)
        (Development|PrintString "Hello")))
    (:then_1
      (if (not (Variables|Default|GetbUseControllerRotationYaw))
        (if (< _returnvalue_3 -91.0)
          (Variables|Default|SetFreeLookChange (+ _returnvalue_3 3.6e+02))
          (elif (> _returnvalue_3 91.0)
            (Variables|Default|SetFreeLookChange (- _returnvalue_3 3.6e+02))
            (else
              (Variables|Default|SetFreeLookChange _returnvalue_3))))))
    (:then_2
      (Utilities|IsValid _item
        (:Is%20Valid
          (if (Utilities|ClassIsChildOf _returnvalue_2 "/Game/Items/Weapons/Guns/BP_Gun.BP_Gun_C")
            (bind _asbp_gun (Utilities|Casting|CastToBP_Gun _item))
            (Default|Equip _asbp_gun)
            (elif (Utilities|ClassIsChildOf _returnvalue_2 "/Game/Items/Building/BP_Building.BP_Building_C")
              (bind _asbp_building (Utilities|Casting|CastToBP_Building _item))
              (bind _output_get (Variables|Default|SetBuilding%20ref _asbp_building))
              (Default|SetUse _output_get true))))))
    (:then_3
      (for _index (range 0 8)
        (if (!= _index (Variables|Inventory|GetHotBarIndex))
          (Utilities|IsValid (Utilities|Array|Get(acopy) (Variables|Inventory|GetInventory) _index)
            (:Is%20Valid
              (if (Utilities|ClassIsChildOf (Utilities|GetClass (Utilities|Array|Get(acopy) (Variables|Inventory|GetInventory) _index)) "/Game/Items/Weapons/Guns/BP_Gun.BP_Gun_C")
                (bind _asbp_gun_2 (Utilities|Casting|CastToBP_Gun (Utilities|Array|Get(acopy) (Variables|Inventory|GetInventory) _index)))
                (Default|Unequip _asbp_gun_2)
                (elif (Utilities|ClassIsChildOf (Utilities|GetClass (Utilities|Array|Get(acopy) (Variables|Inventory|GetInventory) _index)) "/Game/Items/Building/BP_Building.BP_Building_C")
                  (bind _asbp_building_2 (Utilities|Casting|CastToBP_Building (Utilities|Array|Get(acopy) (Variables|Inventory|GetInventory) _index)))
                  (Default|SetUse _asbp_building_2 false))))))))
    (:then_4
      (bind _health (CallFunction|Health 0.0))
      (if (<= _health 0.0)
        (Components|Animation|PlayAnimation (Variables|Character|GetMesh) "/Game/Imports/AnimStarterPack/Death_3.Death_3" false)
        (else
          (Development|PrintString (Utilities|String|ToString(Float) _health) true true "(R=0.000000,G=0.660000,B=1.000000,A=1.000000)" 0.0))))))

(event Input|ActionEvents|InputActionADS
  (params (Key :type Key%20Structure :default "AnyKey"))
  (bind _fpc (Variables|Default|GetFPC))
  (bind _gunitem (Variables|Default|GetGunItem))
  ;[1 1 1] Fps Aiming
  (:Pressed
    (if (and (Variables|CharacterSettings|GetFirstPerson) (not (> (Math|Vector|VectorLength (Transformation|GetVelocity)) 0.0)))
      (Utilities|IsValid _gunitem
        (:Is%20Valid
          (Transformation|SetWorldTransform _fpc (Transformation|GetWorldTransform (Variables|/Game/Items/Weapons/Guns/BP_Gun.BP_Gun_C|GetADSCamera _gunitem)) false false)))))
  (:Released
    (Transformation|SetWorldTransform _fpc (Transformation|GetWorldTransform (Variables|Default|GetFPCR)) false false)))

(event Input|ActionEvents|InputActionBuild
  (params (Key :type Key%20Structure :default "AnyKey"))
  (:Pressed
    (Default|CallBuildTogg)))

(event Input|ActionEvents|InputActionCrouchToggle
  (params (Key :type Key%20Structure :default "AnyKey"))
  ;[1 1 1] Crouche(Toggle)
  (:Pressed
    (if (Utilities|Enum|NotEqual(Enum) (Variables|CharacterInfo|GetStance) "NewEnumerator1")
      (CallFunction|ChangeStance "NewEnumerator1")
      (else
        (CallFunction|ChangeStance "NewEnumerator0")))))

(event Input|ActionEvents|InputActionSprint
  (params (Key :type Key%20Structure :default "AnyKey"))
  ;[0 1 1] Movement
  (:Pressed
    (CallFunction|SetSprinting true))
  (:Released
    (CallFunction|SetSprinting false)))

(event Input|ActionEvents|InputActionJump
  (params (Key :type Key%20Structure :default "AnyKey"))
  ;[0 1 1] Movement
  (:Pressed
    (if (Utilities|Enum|NotEqual(Enum) (Variables|CharacterInfo|GetStance) "NewEnumerator2")
      (Character|Jump)
      (Variables|Util|SetJumped%20Button%20Pressed true)))
  (:Released
    (Character|StopJumping)))

(event Input|ActionEvents|InputActionHotbarUp
  (params (Key :type Key%20Structure :default "AnyKey"))
  ;[1 1 1] Hot Bar Scroll
  (:Pressed
    (CallFunction|SetHotbarIndex (+ (Variables|Inventory|GetHotBarIndex) 1))))

(event Input|ActionEvents|InputActionInteract
  (params (Key :type Key%20Structure :default "AnyKey"))
  ;[1 1 1] Interact
  (:Pressed
    (CallFunction|Interact(Server))))

(event Input|ActionEvents|InputActionReload
  (params (Key :type Key%20Structure :default "AnyKey"))
  (bind _inventory (Variables|Inventory|GetInventory))
  (bind _hotbarindex (Variables|Inventory|GetHotBarIndex))
  (bind _item (Utilities|Array|Get(acopy) _inventory _hotbarindex))
  ;[1 1 1] Reload
  (:Pressed
    (if (Utilities|ClassIsChildOf (Utilities|GetClass _item) "/Game/Items/Weapons/Guns/BP_Gun.BP_Gun_C")
      (bind _asbp_gun (Utilities|Casting|CastToBP_Gun _item))
      (Default|Reload _asbp_gun))))

(event Input|ActionEvents|InputActionHotbarDown
  (params (Key :type Key%20Structure :default "AnyKey"))
  ;[1 1 1] Hot Bar Scroll
  (:Pressed
    (CallFunction|SetHotbarIndex (- (Variables|Inventory|GetHotBarIndex) 1))))

(event Input|ActionEvents|InputActionFire
  (params (Key :type Key%20Structure :default "AnyKey"))
  (bind _hotbarindex (Variables|Inventory|GetHotBarIndex))
  (bind _inventory (Variables|Inventory|GetInventory))
  (bind _item (Utilities|Array|Get(acopy) _inventory _hotbarindex))
  (bind _returnvalue (Utilities|GetClass _item))
  (bind _returnvalue_2 (Utilities|IsValid _item))
  (bind _returnvalue_3 (Utilities|ClassIsChildOf _returnvalue "/Game/Items/Weapons/Guns/BP_Gun.BP_Gun_C"))
  ;[1 1 1] Fire
  (:Pressed
    (Variables|Default|SetFireDown true)
    (if _returnvalue_2
      (if _returnvalue_3
        (bind _asbp_gun (Utilities|Casting|CastToBP_Gun _item))
        (Default|FireWeapon _asbp_gun false)
        (else
          (Default|Action _item)))
      (else
        (CallFunction|FireTrace))))
  (:Released
    (Variables|Default|SetFireDown false)
    (if _returnvalue_2
      (if _returnvalue_3
        (bind _asbp_gun_2 (Utilities|Casting|CastToBP_Gun _item))
        (Default|FireWeapon _asbp_gun_2 true)
        (else
          (Default|Action _item 1))))))

(event Input|ActionEvents|InputActionToggleView
  (params (Key :type Key%20Structure :default "AnyKey"))
  ;[1 1 1] Toggle Camera View
  (:Pressed
    (bind _isa (Utilities|FlowControl|FlipFlop)
      (:A
        (Variables|CharacterSettings|SetFirstPerson _isa)
        (Components|Activation|SetActive (Variables|Default|GetFPC) true false)
        (Components|Activation|SetActive (Variables|Default|GetTPC) false true))
      (:B
        (Variables|CharacterSettings|SetFirstPerson _isa)
        (Components|Activation|SetActive (Variables|Default|GetTPC) true false)
        (Components|Activation|SetActive (Variables|Default|GetFPC) false true)))))

(event Input|ActionEvents|InputActionCrouch
  (params (Key :type Key%20Structure :default "AnyKey"))
  ;[1 1 1] Crouch
  (:Pressed
    (CallFunction|ChangeStance "NewEnumerator1"))
  (:Released
    (CallFunction|ChangeStance "NewEnumerator0")))

(event Input|ActionEvents|InputActionVoice
  (params (Key :type Key%20Structure :default "AnyKey"))
  ;[1 1 1] Voice(Test)
  (:Pressed
    (Class|AdvancedVoiceLibrary|StartNetworkedVoice))
  (:Released
    (Class|AdvancedVoiceLibrary|StopNetworkedVoice)))

(event Input|ActionEvents|InputActionADS
  (params (Key :type Key%20Structure :default "AnyKey"))
  (bind _tpc (Variables|Default|GetTPC))
  ;[1 1 1] Ads
  (:Pressed
    (CallFunction|SetADS true)
    (bind (_direction _alpha) (Timeline|FovFocus PlayFromStart)
      (:Update
        (switch Utilities|FlowControl|Switch|SwitchonETimelineDirection _direction
          (:Forward
            (Camera|SetFieldOfView _tpc (Math|Float|Lerp 9e+01 7e+01 _alpha)))
          (:Backward
            (Camera|SetFieldOfView _tpc (Math|Float|Lerp 9e+01 7e+01 _alpha)))))))
  (:Released
    (CallFunction|SetADS false)
    (Timeline|FovFocus ReverseFromEnd)))

(event Input|ActionEvents|InputActionFire
  (params (Key :type Key%20Structure :default "AnyKey"))
  (:Pressed
    (Default|CallFirePressed)))

(event Input|ActionEvents|InputActionFreeLook
  (params (Key :type Key%20Structure :default "AnyKey"))
  (bind _returnvalue (Game|GetPlayerCameraManager 0))
  (bind _returnvalue_2 (Game|GetPlayerCameraManager 0))
  (bind _returnvalue_3 (Pawn|GetControlRotation :!class /Script/Engine.Pawn))
  (bind _tpc (Variables|Default|GetTPC))
  (bind _returnvalue_4 (Transformation|GetWorldRotation _tpc))
  (bind (_roll _pitch) (Math|Rotator|BreakRotator _returnvalue_3))
  (bind _yaw (Math|Rotator|BreakRotator _returnvalue_4))
  ;[1 1 1] Free Look
  (:Pressed
    (Variables|Default|SetbUseControllerRotationYaw false)
    (Variables|/Script/Engine.PlayerCameraManager|SetViewYawMax _returnvalue_2 (+ _yaw 9e+01))
    (Variables|/Script/Engine.PlayerCameraManager|SetViewYawMin _returnvalue_2 (- _yaw 9e+01))
    (Variables|Util|SetFreeLookSavedRotation (.Yaw (Math|Rotator|BreakRotator (Pawn|GetControlRotation :!class /Script/Engine.Pawn)))))
  (:Released
    (if (or (> (Variables|Default|GetFreeLookChange) 2.0) (< (Variables|Default|GetFreeLookChange) -2.0))
      (bind _alpha (Timeline|Free%20Look%20Rotate%20Back PlayFromStart)
        (:Update
          (Pawn|SetControlRotation (Game|GetPlayerController 0) (Math|Rotator|MakeRotator _roll _pitch (+ (Math|Float|Lerp (Variables|Default|GetFreeLookChange) 0.0 _alpha) (Variables|Util|GetFreeLookSavedRotation)))))
        (:Finished
          (Variables|Default|SetbUseControllerRotationYaw true :!label _label)
          (Variables|/Script/Engine.PlayerCameraManager|SetViewYawMax _returnvalue 359.99)
          (Variables|/Script/Engine.PlayerCameraManager|SetViewYawMin _returnvalue 0.0)))
      (else
        (goto _label)))))

(event Input|AxisEvents|InputAxisMoveForward
  (params (AxisValue :type Float%20%28single-precision%29))
  ;[0 1 1] Movement
  (Pawn|Input|AddMovementInput (Transformation|GetActorForwardVector) AxisValue false)
  (if (== AxisValue 1.0)
    (bind _speed (CallFunction|GetMovementSpeed))
    (CallFunction|SetMovementSpeed _speed)
    (elif (== AxisValue -1.0)
      (bind _speed_2 (CallFunction|GetMovementSpeed))
      (CallFunction|SetMovementSpeed (/ _speed_2 1.5)))))

(event Input|AxisEvents|InputAxisMoveRight
  (params (AxisValue :type Float%20%28single-precision%29))
  ;[0 1 1] Movement
  (Pawn|Input|AddMovementInput (Transformation|GetActorRightVector) AxisValue false))

(event Input|AxisEvents|InputAxisMouseX
  (params (AxisValue :type Float%20%28single-precision%29))
  ;[0 1 1] Movement
  (Pawn|Input|AddControllerYawInput (* AxisValue (Variables|CharacterSettings|GetBaseTurnRate) (Utilities|Time|GetWorldDeltaSeconds))))

(event Input|AxisEvents|InputAxisMouseY
  (params (AxisValue :type Float%20%28single-precision%29))
  ;[0 1 1] Movement
  (Pawn|Input|AddControllerPitchInput (* AxisValue (Variables|CharacterSettings|GetBaseLookUpRate) (Utilities|Time|GetWorldDeltaSeconds))))

(event Input|KeyboardEvents|LeftCtrl
  (params (Key :type Key%20Structure :default "AnyKey")))

(event Input|KeyboardEvents|C
  (params (Key :type Key%20Structure :default "AnyKey"))
  (:Pressed
    (Variables|Default|SetCrouch%20Button%20Down true))
  (:Released
    (Variables|Default|SetCrouch%20Button%20Down false)))

(event Input|KeyboardEvents|LeftCtrl
  (params (Key :type Key%20Structure :default "AnyKey")))

(fn ConstructionScript
  (Utilities|Array|Resize (Variables|Inventory|GetInventory) 39))

(fn GetMovementSpeed
  (bind _movementspeed (Variables|CharacterSettings|GetMovementSpeed))
  (bind _sprinting (Variables|CharacterInfo|GetSprinting))
  (bind (_walking _jogging _sprinting_2 _crouching _prone) (Utilities|Struct|BreakST_Movement_Speed _movementspeed))
  (switch Utilities|FlowControl|Switch|SwitchonEN_Stance_Type (Variables|CharacterInfo|GetStance)
    (:NewEnumerator0
      (switch Utilities|FlowControl|Switch|SwitchonEN_Movement_Type (Variables|CharacterInfo|GetMovementType)
        (:NewEnumerator0
          (if _sprinting
            _
            (else
              (return _walking))))
        (:NewEnumerator1
          (if _sprinting
            _
            (else
              (return _jogging)))))
      (return _sprinting_2))
    (:NewEnumerator1
      (return _crouching))
    (:NewEnumerator2
      (return _prone))
    (:NewEnumerator3
      (return 0.0))))

(fn GetSpacetoAddItem
  (bind (_array_element _array_index) (Utilities|Array|ForEachLoopwithBreak (Variables|Inventory|GetInventory))
    (:LoopBody
      (Utilities|IsValid _array_element
        (:Is%20Not%20Valid
          (return _array_index))))
    (:Completed
      (return -1))))

(fn TestThrowPipe
  (bind _returnvalue (Pawn|GetControlRotation :!class /Script/Engine.Pawn))
  (CallFunction|SpawnActoronServer "/Game/Items/Weapons/Throwable/BP_Throwable.BP_Throwable_C" (Math|Transform|MakeTransform (+ (Transformation|GetActorLocation) (Math|Vector|RotateVector "50.000000,25.000000,100.000000" _returnvalue)) _returnvalue "1,1.000000,1")))

(fn SwitchInventoryItem
  (params (Old :type Integer) (New :type Integer))
  (bind _inventory (Variables|Inventory|GetInventory))
  (bind _item (Utilities|Array|Get(acopy) _inventory Old))
  (bind _item_2 (Utilities|Array|Get(acopy) _inventory New))
  (Utilities|IsValid _item_2
    (:Is%20Valid
      (bind _output_get (LocalVariables|SetItem _item_2))
      (Utilities|Array|SetArrayElem _inventory New _item)
      (Utilities|Array|SetArrayElem _inventory Old _output_get))
    (:Is%20Not%20Valid
      (Utilities|Array|SetArrayElem _inventory New _item)
      (Utilities|Array|SetArrayElem _inventory Old 0))))

(fn OnRepHealth
  (Development|PrintString (Utilities|String|ToString(Float) (Variables|CharacterInfo|GetHealth))))

(fn Location
  (return 0 (Variables|Default|GetBuildLocation_)))

(fn Health
  (params (DMG%20Taken :type Float%20%28single-precision%29))
  (return (- (Variables|CharacterInfo|GetHealth) DMG%20Taken)))