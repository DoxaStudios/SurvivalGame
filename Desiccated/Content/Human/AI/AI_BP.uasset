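; AI controller for human NPCs that runs AI_BT on possession and uses perception to drive player conversation and leader assignment.
; Sensing the player enables talking, so Enter copies the pawn's Question to BP_Huma and opens a Chat widget once.
; Sensing a same-class AI compares Nightcrawler values and calls SetLeader on that pawn when they match.
; Tick prints the blackboard name for debugging.
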(event OnTargetPerceptionUpdated(AIPerception)
  (params (Actor :type Actor%20Object%20Reference) (Stimulus :type AI%20Stimulus%20Structure))
  (Variables|Default|SetActorStimulus Actor)
  (Variables|Default|SetSee (.bSuccessfullySensed (Utilities|Struct|BreakAIStimulus Stimulus)))
  (if (and (== (Game|GetPlayerCharacter 0) Actor) (Variables|Default|GetSee))
    (Utilities|FlowControl|DoOnce false :!label _label
      (:Completed
        (Variables|Default|Setcantalk true)
        (Input|EnableInput (Game|GetPlayerCharacter 0) (Game|GetPlayerController 0))))
    (else
      (Variables|Default|Setcantalk false)
      (Utilities|FlowControl|Sequence
        (:then_0
          (goto _label Reset))
        (:then_1
          (CallFunction|SeeAI))))))

(event Custom|See%20AI
  (bind _returnvalue (AI|GetAIController (Variables|Default|GetActorStimulus)))
  (bind _returnvalue_2 (AI|GetAIController (Variables|Default|GetReference)))
  (if (and (== (Utilities|GetClass _returnvalue_2) (Utilities|GetClass _returnvalue)) (Variables|Default|GetSee))
    (bind _asai (Utilities|Casting|CastToAI (Pawn|GetControlledPawn _returnvalue)))
    (bind _asai_bp (Utilities|Casting|CastToAI_BP _returnvalue))
    (bind _output_get (Variables|AI_BP_C|SetNightcrawler _asai_bp (Variables|/Game/Human/AI/AI.AI_C|GetNightCrawler? _asai)))
    (if (Math|Boolean|Equal(Boolean) _output_get (Variables|Default|GetNightcrawler))
      (Default|SetLeader _asai))))

(event EventOnPossess
  (params (PossessedPawn :type Pawn%20Object%20Reference))
  (AI|RunBehaviorTree "/Game/Human/AI/AI_BT.AI_BT")
  (Variables|Default|SetReference PossessedPawn))

(event EventTick
  (params (DeltaSeconds :type Float%20%28single-precision%29))
  (Development|PrintString (Utilities|GetDisplayName (AI|GetBlackboard 0))))

(event Input|KeyboardEvents|Enter
  (params (Key :type Key%20Structure :default "AnyKey"))
  (bind _reference (Variables|Default|GetReference))
  (:Pressed
    (if (and (not (Variables|Default|Getaskalready?)) (Variables|Default|Getcantalk))
      (bind _asai (Utilities|Casting|CastToAI _reference))
      (bind _asbp_huma (Utilities|Casting|CastToBP_Huma (Game|GetPlayerCharacter 0)))
      (Variables|/Game/Human/BP_Huma.BP_Huma_C|Setchat _asbp_huma (Variables|/Game/Human/AI/AI.AI_C|GetQuestion _asai))
      (Variables|/Game/Human/BP_Huma.BP_Huma_C|Setasker _asbp_huma _reference)
      (Utilities|FlowControl|DoOnce false
        (:Completed
          (Variables|Default|Setaskalready? true)
          (Utilities|FlowControl|Delay 0.5)
          (bind _returnvalue (UserInterface|CreateWidget "/Game/Human/AI/Chat.Chat_C" (Game|GetPlayerController 0)))
          (UserInterface|Viewport|AddtoViewport _returnvalue 0))))))

(fn ConstructionScript)