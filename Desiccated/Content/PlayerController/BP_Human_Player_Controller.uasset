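; Human player controller that owns the player's HUD, menus and chat, and fetches the Steam avatar shown in the inventory widget.
; CreateHud builds inventory, crosshair and chat widgets, binding the inventory to the owned character.
; Input toggles the main menu, debug menu and inventory, with ToggleKeys switching cursor and input mode.
; Outgoing chat goes to DesiccatedMainGameMode, while a RepNotify on ChatMessages pushes the newest message to the chat widget.
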(event Custom|Toggle%20Keys
  (params (Toggle :type Boolean))
  (bind _self self)
  (bind _output_get (Variables|/Script/Engine.PlayerController|SetbShowMouseCursor _self Toggle))
  (bind _output_get_2 (Variables|/Script/Engine.PlayerController|SetbEnableClickEvents _self _output_get))
  (bind _output_get_3 (Variables|/Script/Engine.PlayerController|SetbEnableMouseOverEvents _self _output_get_2))
  (if _output_get_3
    (Input|SetInputModeGameandUI _self 0 false false)
    (else
      (Input|SetInputModeGameOnly _self))))

(event Custom|Send%20Chat%20Message
  (params (Chat :type ST%20Chat%20Struct%20Structure))
  (bind _asdesiccated_main_game_mode (Utilities|Casting|CastToDesiccatedMainGameMode (Game|GetGameMode)))
  (Default|RecieveChat _asdesiccated_main_game_mode Chat))

(event EventBeginPlay
  (bind _returnvalue (Class|AdvancedFriendsLibrary|GetSteamFriendAvatar (Class|AdvancedSessionsLibrary|GetUniqueNetID self) "SteamAvatar_Small"))
  (Variables|Default|SetAvatar _returnvalue))

(event Input|ActionEvents|InputActionInventory
  (params (Key :type Key%20Structure :default "AnyKey"))
  (:Pressed
    (bind _output_get (Variables|Default|SetInventory%20Visible (not (Variables|Default|GetInventory%20Visible))))
    (Default|ViewInventory (Variables|Default|GetInventory%20Widget) (Variables|Default|GetInventory%20Visible))
    (CallFunction|ToggleKeys _output_get)))

(event Input|KeyboardEvents|Escape
  (params (Key :type Key%20Structure :default "AnyKey"))
  (:Pressed
    (bind _output_get (Variables|Default|SetOptions%20Open (not (Variables|Default|GetOptions%20Open))))
    (CallFunction|ToggleKeys _output_get)
    (if _output_get
      (bind _returnvalue (UserInterface|CreateWidget "/Game/Widgets/MainMenu/W_Main_Menu.W_Main_Menu_C"))
      (UserInterface|Viewport|AddtoViewport _returnvalue 0)
      (Variables|Default|SetMain_Menu _returnvalue)
      (Widget|RemovefromParent (Variables|Default|GetInventory%20Widget))
      (else
        (Widget|RemovefromParent (Variables|Default|GetMain_Menu))
        (UserInterface|Viewport|AddtoViewport (Variables|Default|GetInventory%20Widget) 0)))))

(event Input|KeyboardEvents|F3
  (params (Key :type Key%20Structure :default "AnyKey"))
  (:Pressed
    (bind _output_get (Variables|Default|SetDebug (not (Variables|Default|GetDebug))))
    (CallFunction|ToggleKeys _output_get)
    (if _output_get
      (bind _returnvalue (UserInterface|CreateWidget "/Game/Widgets/Debug/W_Debug_Menu.W_Debug_Menu_C"))
      (UserInterface|Viewport|AddtoViewport _returnvalue 0)
      (Variables|Default|SetDebug%20Menu _returnvalue)
      (else
        (Widget|RemovefromParent (Variables|Default|GetDebug%20Menu))))))

(event Input|KeyboardEvents|Q
  (params (Key :type Key%20Structure :default "AnyKey"))
  (:Pressed
    (bind _output_get (Variables|Default|SetOptions%20Open (not (Variables|Default|GetOptions%20Open))))
    (CallFunction|ToggleKeys _output_get)
    (if _output_get
      (bind _returnvalue (UserInterface|CreateWidget "/Game/Widgets/MainMenu/W_Main_Menu.W_Main_Menu_C"))
      (UserInterface|Viewport|AddtoViewport _returnvalue 0)
      (Variables|Default|SetMain_Menu _returnvalue)
      (Widget|RemovefromParent (Variables|Default|GetInventory%20Widget))
      (else
        (Widget|RemovefromParent (Variables|Default|GetMain_Menu))
        (UserInterface|Viewport|AddtoViewport (Variables|Default|GetInventory%20Widget) 0)))))

(fn ConstructionScript)

(fn CreateHud
  (bind _returnvalue (UserInterface|CreateWidget "/Game/Widgets/Inventory/W_Inventory.W_Inventory_C"))
  (UserInterface|Viewport|AddtoViewport _returnvalue 0)
  (Variables|Default|SetInventory%20Widget _returnvalue)
  (Variables|/Game/Widgets/Inventory/W_Inventory.W_Inventory_C|Setimage _returnvalue (Variables|Default|GetAvatar))
  (Default|SetCharacter _returnvalue (Variables|Default|GetOwned%20Character))
  (Default|ViewInventory _returnvalue false)
  (bind _returnvalue_2 (UserInterface|CreateWidget "/Game/Widgets/Crosshair/W_Crosshair.W_Crosshair_C"))
  (UserInterface|Viewport|AddtoViewport _returnvalue_2 0)
  (bind _returnvalue_3 (UserInterface|CreateWidget "/Game/Widgets/ChatSystem/W_ChatInterface.W_ChatInterface_C"))
  (Variables|Chat|SetChat%20Widget _returnvalue_3)
  (UserInterface|Viewport|AddtoViewport _returnvalue_3 0))

(fn OnRepChatMessages
  (bind _chat_messages (Variables|Chat|GetChat%20Messages))
  (bind _chat_widget (Variables|Chat|GetChat%20Widget))
  (Utilities|IsValid _chat_widget
    (:Is%20Valid
      (Default|ChatMessage _chat_widget (Utilities|Array|Get(acopy) _chat_messages (Utilities|Array|LastIndex _chat_messages))))))