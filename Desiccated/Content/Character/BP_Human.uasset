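; Player-controlled human character with first/third-person view toggle, stances, sprinting, aiming, voice chat and item interaction.
; Input feeds state and server-named events: movement speed follows stance and sprint, while a camera trace picks items into an inventory array whose hotbar slot handles firing.
; Tick creates inventory and crosshair widgets once locally controlled, and tracks wrapped free-look yaw, which a timeline eases back on release.
; Includes debug prints and a test throwable spawner.
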(event Custom|Set%20Combat%20Mode
  (params (Combat%20Mode :type Boolean))
  (Variables|CharacterInfo|SetCombatMode Combat%20Mode))

(event Custom|Set%20ADS
  (params (ADS :type Boolean))
  (Variables|CharacterInfo|SetADS ADS))

(event Custom|Interact%28Server%29
  (bind _camera (Variables|Default|GetCamera))
  (bind _returnvalue (Transformation|GetWorldLocation _camera))
  (bind _outhit (Collision|LineTraceByChannel _returnvalue (+ _returnvalue (* (Math|Vector|GetForwardVector _camera) (+ (Variables|/Script/Engine.SpringArmComponent|GetTargetArmLength (Variables|Default|GetArm)) (Variables|Util|GetInteract%20Distance)))) "TraceTypeQuery1" false 0 "Persistent"))
  (if (Utilities|ClassIsChildOf (Utilities|GetClass (.HitActor (Collision|BreakHitResult _outhit))) "/Game/Items/Item.Item_C")
    (bind _asitem (Utilities|Casting|CastToItem (.HitActor (Collision|BreakHitResult _outhit))))
    (bind _index (CallFunction|GetSpacetoAddItem))
    (if (!= _index -1)
      (Utilities|Array|SetArrayElem (Variables|Inventory|GetInventory) _index _asitem)
      (Default|Pickup _asitem self))))

(event Custom|Toggle%20Keys
  (params (Toggle :type Boolean))
  (bind _returnvalue (Game|GetPlayerController 0))
  (bind _returnvalue_2 (Game|GetPlayerController 0))
  (bind _output_get (Variables|/Script/Engine.PlayerController|SetbShowMouseCursor _returnvalue Toggle))
  (bind _output_get_2 (Variables|/Script/Engine.PlayerController|SetbEnableClickEvents _returnvalue _output_get))
  (bind _output_get_3 (Variables|/Script/Engine.PlayerController|SetbEnableMouseOverEvents _returnvalue _output_get_2))
  (if _output_get_3
    (Input|SetInputModeGameandUI _returnvalue_2 0 false false)
    (else
      (Input|SetInputModeGameOnly _returnvalue_2))))

(event Custom|Create%20Hud
  ;[1 1 1] Create HUD
  (bind _returnvalue (UserInterface|CreateWidget "/Game/Widgets/Inventory/W_Inventory.W_Inventory_C"))
  (UserInterface|Viewport|AddtoViewport _returnvalue 0)
  (Variables|Inventory|SetInventoryWidget _returnvalue)
  (Default|SetCharacter _returnvalue self)
  (Default|ViewInventory _returnvalue false)
  (bind _returnvalue_2 (UserInterface|CreateWidget "/Game/Widgets/Crosshair/W_Crosshair.W_Crosshair_C"))
  (UserInterface|Viewport|AddtoViewport _returnvalue_2 0)
  (Variables|Default|SetCrosshair%20Widget _returnvalue_2))

(event Custom|Server%20Switch%20View
  (params (First%20Person :type Boolean))
  (bind _arm (Variables|Default|GetArm))
  ;[1 1 1] Toggle Camera View
  (if First%20Person
    (Variables|/Script/Engine.SpringArmComponent|SetTargetArmLength _arm 3e+02)
    (else
      (Variables|/Script/Engine.SpringArmComponent|SetTargetArmLength _arm 0.0))))

(event Custom|Set%20Hotbar%20Index
  (params (Index :type Integer))
  (if (== Index -1)
    (Variables|Inventory|SetHotBarIndex 6)
    (elif (== Index 7)
      (Variables|Inventory|SetHotBarIndex 0)
      (else
        (Variables|Inventory|SetHotBarIndex Index)))))

(event Custom|Spawn%20Actor%20On%20Server
  (params (Actor :type Actor%20Class%20Reference) (Transform :type Transform))
  (Game|SpawnActorfromClass Actor Transform "Undefined" 0 0))

(event Custom|Set%20Sprinting
  (params (Sprinting :type Boolean))
  (Variables|CharacterInfo|SetSprinting Sprinting))

(event Custom|Set%20Movement%20Speed
  (params (Speed :type Float%20%28single-precision%29))
  ;[0 1 1] Movement
  (Variables|/Script/Engine.CharacterMovementComponent|SetMaxWalkSpeed (Variables|Character|GetCharacterMovement) Speed))

(event Custom|Change%20Equiped)

(event Custom|Change%20Stance
  (params (Stance :type EN_Stance_Type%20Enum))
  (Variables|CharacterInfo|SetStance Stance))

(event Game|Damage|EventAnyDamage
  (params (Damage :type Float%20%28single-precision%29) (DamageType :type Damage%20Type%20Object%20Reference) (InstigatedBy :type Controller%20Object%20Reference) (DamageCauser :type Actor%20Object%20Reference))
  (Development|PrintString "Hello"))

(event EventBeginPlay
  (bind _returnvalue (Game|GetPlayerCameraManager 0))
  (Variables|/Script/Engine.PlayerCameraManager|SetViewPitchMax _returnvalue 8e+01)
  (Variables|/Script/Engine.PlayerCameraManager|SetViewPitchMin _returnvalue -7e+01))

(event EventTick
  (params (DeltaSeconds :type Float%20%28single-precision%29))
  (bind _returnvalue (Pawn|GetControlRotation :!class /Script/Engine.Pawn))
  (bind _freelooksavedrotation (Variables|Util|GetFreeLookSavedRotation))
  (bind _yaw (Math|Rotator|BreakRotator _returnvalue))
  (bind _returnvalue_2 (- _yaw _freelooksavedrotation))
  (Utilities|FlowControl|Sequence
    (:then_0
      (Utilities|IsControlled
        (:True
          (Utilities|FlowControl|DoOnce false
            (:Completed
              (CallFunction|CreateHud))))))
    (:then_1
      (if (not (Variables|Default|GetbUseControllerRotationYaw))
        (if (< _returnvalue_2 -91.0)
          (Variables|Default|SetFreeLookChange (+ _returnvalue_2 3.6e+02))
          (elif (> _returnvalue_2 91.0)
            (Variables|Default|SetFreeLookChange (- _returnvalue_2 3.6e+02))
            (else
              (Variables|Default|SetFreeLookChange _returnvalue_2))))))))

(event Input|ActionEvents|InputActionSprint
  (params (Key :type Key%20Structure :default "AnyKey"))
  ;[0 1 1] Movement
  (:Pressed
    (CallFunction|SetSprinting true))
  (:Released
    (CallFunction|SetSprinting false)))

(event Input|ActionEvents|InputActionJump
  (params (Key :type Key%20Structure :default "AnyKey"))
  ;[0 1 1] Movement
  (:Pressed
    (if (Utilities|Enum|NotEqual(Enum) (Variables|CharacterInfo|GetStance) "NewEnumerator2")
      (Character|Jump)
      (Variables|Util|SetJumped%20Button%20Pressed true)))
  (:Released
    (Character|StopJumping)))

(event Input|ActionEvents|InputActionHotbarUp
  (params (Key :type Key%20Structure :default "AnyKey"))
  ;[1 1 1] Hot Bar Scroll
  (:Pressed
    (CallFunction|SetHotbarIndex (+ (Variables|Inventory|GetHotBarIndex) 1))))

(event Input|ActionEvents|InputActionInventory
  (params (Key :type Key%20Structure :default "AnyKey"))
  (:Pressed
    (bind _output_get (Variables|Inventory|SetInventoryVisible (not (Variables|Inventory|GetInventoryVisible))))
    (Default|ViewInventory (Variables|Inventory|GetInventoryWidget) _output_get)
    (CallFunction|ToggleKeys _output_get)))

(event Input|ActionEvents|InputActionInteract
  (params (Key :type Key%20Structure :default "AnyKey"))
  (:Pressed
    (CallFunction|Interact(Server))))

(event Input|ActionEvents|InputActionHotbarDown
  (params (Key :type Key%20Structure :default "AnyKey"))
  ;[1 1 1] Hot Bar Scroll
  (:Pressed
    (CallFunction|SetHotbarIndex (- (Variables|Inventory|GetHotBarIndex) 1))))

(event Input|ActionEvents|InputActionCrouchToggle
  (params (Key :type Key%20Structure :default "AnyKey"))
  (:Pressed
    (if (Utilities|Enum|NotEqual(Enum) (Variables|CharacterInfo|GetStance) "NewEnumerator1")
      (CallFunction|ChangeStance "NewEnumerator1")
      (else
        (CallFunction|ChangeStance "NewEnumerator0")))))

(event Input|ActionEvents|InputActionFire
  (params (Key :type Key%20Structure :default "AnyKey"))
  (bind _hotbarindex (Variables|Inventory|GetHotBarIndex))
  (bind _inventory (Variables|Inventory|GetInventory))
  (bind _item (Utilities|Array|Get(acopy) _inventory _hotbarindex))
  (bind _returnvalue (Utilities|IsValid _item))
  ;[1 1 1] Fire
  (:Pressed
    (if _returnvalue
      (Default|Action _item)
      (Development|PrintString "2323o")))
  (:Released
    (if _returnvalue
      (Default|Action _item 1))))

(event Input|ActionEvents|InputActionToggleView
  (params (Key :type Key%20Structure :default "AnyKey"))
  (bind _arms (Variables|Default|GetArms))
  (bind _mesh (Variables|Character|GetMesh))
  (bind _arm (Variables|Default|GetArm))
  ;[1 1 1] Toggle Camera View
  (:Pressed
    (if (Variables|CharacterSettings|GetFirstPerson)
      (Variables|/Script/Engine.SpringArmComponent|SetTargetArmLength _arm 3e+02)
      (Rendering|Material|SetMaterial _mesh 1 "/Game/Soldiers/USA/UsaSoldier2/M_UsaSoldier2_Head.M_UsaSoldier2_Head")
      (Rendering|SetVisibility _arms false false)
      (else
        (Variables|/Script/Engine.SpringArmComponent|SetTargetArmLength _arm 0.0)
        (Rendering|Material|SetMaterial _mesh 1 "/Game/Soldiers/M_InvisibleHead.M_InvisibleHead")
        (Rendering|SetVisibility _arms true false)))
    (CallFunction|ServerSwitchView (Variables|CharacterSettings|GetFirstPerson))
    (Variables|CharacterSettings|SetFirstPerson (not (Variables|CharacterSettings|GetFirstPerson)))))

(event Input|ActionEvents|InputActionProneToggle
  (params (Key :type Key%20Structure :default "AnyKey"))
  (:Pressed
    (if (Utilities|Enum|NotEqual(Enum) (Variables|CharacterInfo|GetStance) "NewEnumerator2")
      (CallFunction|ChangeStance "NewEnumerator2")
      (else
        (CallFunction|ChangeStance "NewEnumerator0")))))

(event Input|ActionEvents|InputActionVoice
  (params (Key :type Key%20Structure :default "AnyKey"))
  (:Pressed
    (Class|AdvancedVoiceLibrary|StartNetworkedVoice))
  (:Released
    (Class|AdvancedVoiceLibrary|StopNetworkedVoice)))

(event Input|ActionEvents|InputActionADS
  (params (Key :type Key%20Structure :default "AnyKey"))
  (bind _crosshair_widget (Variables|Default|GetCrosshair%20Widget))
  (:Pressed
    (CallFunction|SetADS true)
    (Default|ADS _crosshair_widget false))
  (:Released
    (CallFunction|SetADS false)
    (Default|ADS _crosshair_widget true)))

(event Input|ActionEvents|InputActionFreeLook
  (params (Key :type Key%20Structure :default "AnyKey"))
  (bind _returnvalue (Game|GetPlayerCameraManager 0))
  (bind _returnvalue_2 (Game|GetPlayerCameraManager 0))
  (bind _returnvalue_3 (Pawn|GetControlRotation :!class /Script/Engine.Pawn))
  (bind _arm (Variables|Default|GetArm))
  (bind _returnvalue_4 (Transformation|GetWorldRotation _arm))
  (bind (_roll _pitch) (Math|Rotator|BreakRotator _returnvalue_3))
  (bind _yaw (Math|Rotator|BreakRotator _returnvalue_4))
  (:Pressed
    (Variables|Default|SetbUseControllerRotationYaw false)
    (Variables|/Script/Engine.PlayerCameraManager|SetViewYawMax _returnvalue_2 (+ _yaw 9e+01))
    (Variables|/Script/Engine.PlayerCameraManager|SetViewYawMin _returnvalue_2 (- _yaw 9e+01))
    (Variables|Util|SetFreeLookSavedRotation (.Yaw (Math|Rotator|BreakRotator (Pawn|GetControlRotation :!class /Script/Engine.Pawn)))))
  (:Released
    (if (or (> (Variables|Default|GetFreeLookChange) 2.0) (< (Variables|Default|GetFreeLookChange) -2.0))
      (bind _alpha (Timeline|Free%20Look%20Rotate%20Back PlayFromStart)
        (:Update
          (Pawn|SetControlRotation (Game|GetPlayerController 0) (Math|Rotator|MakeRotator _roll _pitch (+ (Math|Float|Lerp (Variables|Default|GetFreeLookChange) 0.0 _alpha) (Variables|Util|GetFreeLookSavedRotation)))))
        (:Finished
          (Variables|Default|SetbUseControllerRotationYaw true :!label _label)
          (Variables|/Script/Engine.PlayerCameraManager|SetViewYawMax _returnvalue 359.99)
          (Variables|/Script/Engine.PlayerCameraManager|SetViewYawMin _returnvalue 0.0)))
      (else
        (goto _label)))))

(event Input|AxisEvents|InputAxisMoveForward
  (params (AxisValue :type Float%20%28single-precision%29))
  ;[0 1 1] Movement
  (Pawn|Input|AddMovementInput (Transformation|GetActorForwardVector) AxisValue false)
  (if (== AxisValue 1.0)
    (bind _speed (CallFunction|GetMovementSpeed))
    (CallFunction|SetMovementSpeed _speed)
    (elif (== AxisValue -1.0)
      (bind _speed_2 (CallFunction|GetMovementSpeed))
      (CallFunction|SetMovementSpeed (/ _speed_2 1.5)))))

(event Input|AxisEvents|InputAxisMoveRight
  (params (AxisValue :type Float%20%28single-precision%29))
  ;[0 1 1] Movement
  (Pawn|Input|AddMovementInput (Transformation|GetActorRightVector) AxisValue false))

(event Input|AxisEvents|InputAxisMouseX
  (params (AxisValue :type Float%20%28single-precision%29))
  ;[0 1 1] Movement
  (Pawn|Input|AddControllerYawInput (* AxisValue (Variables|CharacterSettings|GetBaseTurnRate) (Utilities|Time|GetWorldDeltaSeconds))))

(event Input|AxisEvents|InputAxisMouseY
  (params (AxisValue :type Float%20%28single-precision%29))
  ;[0 1 1] Movement
  (Pawn|Input|AddControllerPitchInput (* AxisValue (Variables|CharacterSettings|GetBaseLookUpRate) (Utilities|Time|GetWorldDeltaSeconds))))

(event Input|KeyboardEvents|G
  (params (Key :type Key%20Structure :default "AnyKey"))
  (:Pressed
    (Development|PrintString (Variables|/Script/Engine.PlayerState|GetPlayerName (Variables|GetPlayerState)))))

(event Input|KeyboardEvents|F
  (params (Key :type Key%20Structure :default "AnyKey"))
  (:Pressed
    (bind _returnvalue (Utilities|Time|SetTimerbyFunctionName self "Test_Throw_Pipe" 0.05 true)))
  (:Released
    (Utilities|Time|PauseTimerbyHandle _returnvalue)))

(fn ConstructionScript
  (Utilities|Array|Resize (Variables|Inventory|GetInventory) 35))

(fn GetMovementSpeed
  (bind _movementspeed (Variables|CharacterSettings|GetMovementSpeed))
  (bind _sprinting (Variables|CharacterInfo|GetSprinting))
  (bind (_walking _jogging _sprinting_2 _crouching _prone) (Utilities|Struct|BreakST_Movement_Speed _movementspeed))
  (switch Utilities|FlowControl|Switch|SwitchonEN_Stance_Type (Variables|CharacterInfo|GetStance)
    (:NewEnumerator0
      (switch Utilities|FlowControl|Switch|SwitchonEN_Movement_Type (Variables|CharacterInfo|GetMovementType)
        (:NewEnumerator0
          (if _sprinting
            _
            (else
              (return _walking))))
        (:NewEnumerator1
          (if _sprinting
            _
            (else
              (return _jogging)))))
      (return _sprinting_2))
    (:NewEnumerator1
      (return _crouching))
    (:NewEnumerator2
      (return _prone))
    (:NewEnumerator3
      (return 0.0))))

(fn GetSpacetoAddItem
  (bind (_array_element _array_index) (Utilities|Array|ForEachLoopwithBreak (Variables|Inventory|GetInventory))
    (:LoopBody
      (Utilities|IsValid _array_element
        (:Is%20Not%20Valid
          (return _array_index))))
    (:Completed
      (return -1))))

(fn TestThrowPipe
  (bind _returnvalue (Pawn|GetControlRotation :!class /Script/Engine.Pawn))
  (CallFunction|SpawnActoronServer "/Game/Items/Weapons/Throwable/BP_Throwable.BP_Throwable_C" (Math|Transform|MakeTransform (+ (Transformation|GetActorLocation) (Math|Vector|RotateVector "50.000000,25.000000,100.000000" _returnvalue)) _returnvalue)))