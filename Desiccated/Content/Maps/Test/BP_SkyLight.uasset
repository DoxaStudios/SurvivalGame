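; Test-map day/night cycle Blueprint that drives the sun, skylight, atmospheric fog and skydome from a clock.
; BeginPlay converts the day length in minutes to seconds per in-game hour, and Tick advances and wraps the hour, printing it each frame.
; Daytime hours turn on sunlight and fog, night turns both off, and the skylight keeps the same intensity.
; The hour also sets the sun's pitch before the skydome updates its sun direction.
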(event EventBeginPlay
  (bind _output_get (Variables|Default|SetOneDay (* (Variables|Default|GetDayLengthInMinutes) 6e+01)))
  (Variables|Default|SetOneHour (/ _output_get 24.0)))

(event Collision|EventActorBeginOverlap
  (params (OtherActor :type Actor%20Object%20Reference)))

(event EventTick
  (params (DeltaSeconds :type Float%20%28single-precision%29))
  (bind _sun (Variables|Default|GetSun))
  (bind _atmosphericfog (Variables|Default|GetAtmosphericFog))
  (bind _skylight (Variables|Default|GetSkylight))
  (bind _lightcomponent (Variables|/Script/Engine.SkyLight|GetLightComponent _skylight))
  (bind _lightcomponent_2 (Variables|/Script/Engine.Light|GetLightComponent _sun))
  (bind _output_get (Variables|Default|SetHour (+ (Variables|Default|GetHour) (/ DeltaSeconds (Variables|Default|GetOneHour)))))
  (if (>= _output_get 24.0)
    (Variables|Default|SetHour 0.0))
  (Development|PrintString (Utilities|String|ToString(Float) _output_get))
  (if (Math|Float|InRange(Float) _output_get 6.0 18.0)
    (Rendering|Components|Light|SetIntensity _lightcomponent_2 1e+01)
    (Rendering|Components|Light|SetIntensity _lightcomponent 1.0)
    (Rendering|SetVisibility _atmosphericfog true false)
    (else
      (Rendering|Components|Light|SetIntensity _lightcomponent_2 0.0)
      (Rendering|Components|Light|SetIntensity _lightcomponent 1.0)
      (Rendering|SetVisibility _atmosphericfog false false)))
  (bind _output_get_2 (Variables|Default|SetSunAngle (+ (* (/ _output_get 6.0) 9e+01) 9e+01)))
  (Transformation|SetActorRotation (Variables|Default|GetSun) (Math|Rotator|MakeRotator 0.0 _output_get_2 0.0))
  (Default|UpdateSunDirection (Variables|Default|GetSkydome)))

(fn ConstructionScript)