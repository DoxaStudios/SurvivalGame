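; Survival game mode that keeps the server-side chat log and announces players joining.
; RecieveChat appends each message to the Messages array, then copies the whole array into ChatMessages on every human player controller in the world.
; PostLogin prints a connection notice with the player's name and sends it through RecieveChat as a Server message.
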(event Custom|Recieve%20Chat
  (params (Chat%20Struct :type ST%20Chat%20Struct%20Structure))
  (Utilities|Array|Add (Variables|Default|GetMessages) Chat%20Struct)
  (bind _outactors (Actor|GetAllActorsOfClass "/Game/PlayerController/BP_Human_Player_Controller.BP_Human_Player_Controller_C"))
  (for _array_element _outactors
    (Variables|/Game/PlayerController/BP_Human_Player_Controller.BP_Human_Player_Controller_C|SetChat%20Messages _array_element (Variables|Default|GetMessages))))

(event EventPostLogin
  (params (NewPlayer :type Player%20Controller%20Object%20Reference))
  (bind _asbp_human_player_controller (Utilities|Casting|CastToBP_Human_Player_Controller NewPlayer))
  (Development|PrintString (Utilities|String|Append "Player " (Class|AdvancedSessionsLibrary|GetPlayerName _asbp_human_player_controller) " has connected!") true true "(R=0.000000,G=0.000000,B=0.000000,A=1.000000)")
  (CallFunction|RecieveChat (Utilities|Struct|MakeST_ChatStruct 0 "Server" (Utilities|Text|ToText(String) (Utilities|String|Append "Player " (Class|AdvancedSessionsLibrary|GetPlayerName _asbp_human_player_controller) " has connected!")) "0001.01.01-00.00.00" "NewEnumerator2")))

(event EventBeginPlay)

(event EventOnLogout
  (params (ExitingController :type Controller%20Object%20Reference)))

(fn ConstructionScript)