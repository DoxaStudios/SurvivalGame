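; Pickup item actor that can be taken out of the world and dropped back in front of its owner.
; Pickup hides the mesh and disables its collision without destroying the actor.
; Drop restores visibility and collision, then moves both actor and mesh a short distance along the owner's forward vector, with sweep and teleport.
; Interaction switches on its type but has no branches wired, and Tick is empty.
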(event Custom|Pickup
  (bind _mesh (Variables|Default|GetMesh))
  (Development|SetHiddeninGame _mesh true false)
  (Collision|SetCollisionEnabled _mesh "NoCollision"))

(event Custom|Drop
  (bind _returnvalue (Components|GetOwner))
  (bind _mesh (Variables|Default|GetMesh))
  (bind _returnvalue_2 (Transformation|GetActorLocation _returnvalue))
  (bind _returnvalue_3 (Transformation|GetActorForwardVector _returnvalue))
  (bind _returnvalue_4 (* _returnvalue_3 1e+02))
  (bind _returnvalue_5 (+ _returnvalue_2 _returnvalue_4))
  (Development|SetHiddeninGame _mesh false false)
  (Collision|SetCollisionEnabled _mesh "QueryAndPhysics")
  (Transformation|SetActorLocation _returnvalue_5 true true)
  (Transformation|SetWorldLocation (Variables|Default|GetMesh) _returnvalue_5 true true))

(event Custom|Interaction
  (params (Type :type Integer))
  (switch int Type))

(event EventTick
  (params (DeltaSeconds :type Float%20%28single-precision%29)))

(fn ConstructionScript
  (|CallParentFunction))