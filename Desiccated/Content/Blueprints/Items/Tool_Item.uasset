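; Tool item Blueprint with a Mine event, apparently an unfinished mining action for the owning character.
; Mine only casts the owner to DesiccatedCharacter and does nothing further.
; A disconnected draft holds a 400-unit Visibility line trace from the character's camera along control rotation, with a check for Minable hit actors, but it never runs and its branch is empty.
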(event Custom|Mine
  (bind _asdesiccated_character (Utilities|Casting|CastToDesiccatedCharacter (Components|GetOwner))))

(event EventBeginPlay)

(event EventActorBeginOverlap
  (params (OtherActor :type Actor%20Object%20Reference)))

(event EventTick
  (params (DeltaSeconds :type Float%20%28single-precision%29)))

(fn ConstructionScript
  (|CallParentFunction))