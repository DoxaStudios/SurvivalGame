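; RCXD projectile that, judging by its input bindings, is an early attempt at a controllable deployable.
; A collision hit or the F key creates an RCXD widget, never added to the viewport, and enables input on the projectile.
; Its axis events drive player character 0 along the projectile's vectors, with both mouse axes adding yaw.
; Branch conditions are constant true, so the stop-movement path never runs.
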(event OnComponentHit(Collision)
  (params (OtherActor :type Actor%20Object%20Reference) (OtherComp :type Primitive%20Component%20Object%20Reference) (NormalImpulse :type Vector :default "0, 0, 0") (Hit :type Hit%20Result%20Structure%20%28by%20ref%29))
  (if true
    (if true
      (UserInterface|CreateWidget "/Game/Blueprints/Widgers/RCXD/RCXD.RCXD_C")
      (Input|EnableInput (Game|GetPlayerController 0))
      (else
        (Components|Movement|StopMovementImmediately (Variables|Default|GetProjectileMovement))))))

(event Input|AxisEvents|InputAxisMoveForward
  (params (AxisValue :type Float%20%28single-precision%29))
  (Pawn|Input|AddMovementInput (Game|GetPlayerCharacter 0) (Transformation|GetActorForwardVector) AxisValue false))

(event Input|AxisEvents|InputAxisMoveRight
  (params (AxisValue :type Float%20%28single-precision%29))
  (Pawn|Input|AddMovementInput (Game|GetPlayerCharacter 0) (Transformation|GetActorRightVector) AxisValue false))

(event Input|AxisEvents|InputAxisMouseX
  (params (AxisValue :type Float%20%28single-precision%29))
  (Pawn|Input|AddControllerYawInput (Game|GetPlayerCharacter 0) (* AxisValue (Variables|Default|GetBaseTurnRate) (Utilities|Time|GetWorldDeltaSeconds))))

(event Input|AxisEvents|InputAxisMouseY
  (params (AxisValue :type Float%20%28single-precision%29))
  (Pawn|Input|AddControllerYawInput (Game|GetPlayerCharacter 0) (* AxisValue (Variables|Default|GetBaseLookUpRate) (Utilities|Time|GetWorldDeltaSeconds))))

(event Input|KeyboardEvents|F
  (params (Key :type Key%20Structure :default "AnyKey"))
  (:Pressed
    (if true
      (UserInterface|CreateWidget "/Game/Blueprints/Widgers/RCXD/RCXD.RCXD_C")
      (Input|EnableInput (Game|GetPlayerController 0))
      (else
        (Components|Movement|StopMovementImmediately (Variables|Default|GetProjectileMovement))))))

(fn ConstructionScript
  (|CallParentFunction))