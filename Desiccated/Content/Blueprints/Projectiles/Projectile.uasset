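; Projectile actor that deals damage to characters it hits.
; When its Collision component hits, it checks for exactly DesiccatedCharacter, or otherwise for a child class of BaseCharecter.
; A match is cast and receives the projectile's Damage through its ApplyDamage call with a fixed damage type, then the projectile destroys itself.
; Hits on any other actor are ignored, leaving the projectile alive.
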(event OnComponentHit(Collision)
  (params (OtherActor :type Actor%20Object%20Reference) (OtherComp :type Primitive%20Component%20Object%20Reference) (NormalImpulse :type Vector :default "0, 0, 0") (Hit :type Hit%20Result%20Structure%20%28by%20ref%29))
  (bind _hitactor (Collision|BreakHitResult Hit))
  (bind _returnvalue (Utilities|GetClass _hitactor))
  (if (== _returnvalue "/Game/Blueprints/Character/DesiccatedCharacter.DesiccatedCharacter_C")
    (bind _asdesiccated_character (Utilities|Casting|CastToDesiccatedCharacter _hitactor))
    (Default|ApplyDamage _asdesiccated_character (Variables|Default|GetDamage) "NewEnumerator1")
    (Actor|DestroyActor :!label _label)
    (elif (Utilities|ClassIsChildOf _returnvalue "/Game/Blueprints/Character/BaseCharecter.BaseCharecter_C")
      (bind _asbase_charecter (Utilities|Casting|CastToBaseCharecter _hitactor))
      (Default|ApplyDamage _asbase_charecter (Variables|Default|GetDamage) "NewEnumerator1")
      (goto _label))))

(fn ConstructionScript)