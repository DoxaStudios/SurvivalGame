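; Base character Blueprint that handles incoming damage through an ApplyDamage event switched on damage type.
; Projectile hits, the only handled type, subtract Health and set a bleeding flag plus a percentage derived from the damage, neither used further here.
; As written, when Health remains at or above zero after the hit, it destroys the mesh and capsule components and prints the damage taken.
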(event Custom|Apply%20Damage
  (params (Damage%20Ammount :type Float%20%28single-precision%29) (Damage%20Type :type Damage_Type%20Enum))
  (switch Utilities|FlowControl|Switch|SwitchonDamage_Type Damage%20Type
    (:NewEnumerator1
      (Variables|Default|SetHealth (- (Variables|Default|GetHealth) Damage%20Ammount))
      (Variables|Default|SetBleeding true)
      (Variables|Default|SetBleedingPercent (/ (/ Damage%20Ammount 2.0) 1e+02))
      (if (>= (Variables|Default|Gethealth) 0.0)
        (Components|DestroyComponent (Variables|Character|GetMesh))
        (Components|DestroyComponent (Variables|Collision|GetCapsuleComponent))
        (Development|PrintString (Utilities|String|Append "Damage Take: " (Utilities|String|ToString(Float) Damage%20Ammount)))))))

(fn ConstructionScript)