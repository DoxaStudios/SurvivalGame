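; Game instance for Desiccated that manages multiplayer sessions and switches between main menu, server list, loading, playing and error screens.
; A StateTransition macro cleans up the current state by hiding widgets or destroying the session, then each screen lazily creates and shows its widget.
; Hosting opens the Colton level on session creation, and joining takes a server-list result.
; Session, network and travel failures feed DisplayError, which destroys the session and shows a dialog.
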(event Custom|DestroySessCaller
  ;[1 1 1] Destroy the session
  (|DestroySession (Game|GetPlayerController 0)))

(event Custom|HostGameEvent
  ;[1 1 1] Host a game session
  (CallFunction|ShowLoadScreen)
  (|AdvancedSession 0 (Game|GetPlayerController 0) 5 0 (Variables|Default|GetenableLan) true false true true false true false true
    (:OnSuccess
      (Game|OpenLevel(byName) "Colton" true "listen"))
    (:OnFailure
      (Utilities|DisplayError "Error: Could not create session"))))

(event Custom|ShowLoadScreen
  (Utilities|StateTransition "NewEnumerator6"
    (:NewState
      (Utilities|IsValid (Variables|Default|Getloading)
        (:Is%20Valid
          _)
        (:Is%20Not%20Valid
          (bind _returnvalue (UserInterface|CreateWidget "/Game/Networking/Widgets/W_Loading.W_Loading_C" (Game|GetPlayerController 0)))
          (bind _output_get (Variables|Default|Setloading _returnvalue))))
      (UserInterface|Viewport|AddtoViewport _returnvalue 0)
      (Input|SetInputModeUIOnly (Game|GetPlayerController 0) _output_get false))))

(event Custom|Show%20Main%20Menu
  (if (Utilities|Enum|Equal(Enum) (Variables|Default|GetCurrent%20State) "NewEnumerator2")
    (Game|OpenLevel(byName) "mainMenu"))
  (Utilities|StateTransition "NewEnumerator1"
    (:NewState
      (Utilities|IsValid (Variables|Default|GetmainMenu)
        (:Is%20Valid
          _)
        (:Is%20Not%20Valid
          (bind _returnvalue (UserInterface|CreateWidget "/Game/Widgets/MainMenu/W_Main_Menu.W_Main_Menu_C" (Game|GetPlayerController 0)))
          (bind _output_get (Variables|Default|SetmainMenu _returnvalue))))
      (Input|SetInputModeUIOnly (Game|GetPlayerController 0) _output_get false)
      (UserInterface|Viewport|AddtoViewport _returnvalue 0))))

(event Custom|Show%20Server%20List
  (bind _returnvalue (Game|GetPlayerController 0))
  (Utilities|StateTransition "NewEnumerator4"
    (:NewState
      (Utilities|IsValid (Variables|Default|GetserverList)
        (:Is%20Valid
          _)
        (:Is%20Not%20Valid
          (bind _returnvalue_2 (UserInterface|CreateWidget "/Game/Networking/Widgets/W_ServerList.W_ServerList_C" _returnvalue))
          (bind _output_get (Variables|Default|SetserverList _returnvalue_2))))
      (UserInterface|Viewport|AddtoViewport _output_get 0)
      (Input|SetInputModeUIOnly _returnvalue _output_get false))))

(event Custom|JoinFromServerList
  (params (SearchResult :type Blueprint%20Session%20Result%20Structure))
  (CallFunction|ShowLoadScreen)
  (|JoinSession (Game|GetPlayerController 0) SearchResult
    (:OnSuccess
      (Development|PrintString "suc"))
    (:OnFailure
      (Utilities|DisplayError "Error: Failed to join server"))))

(event EventHandleNetworkError
  (params (FailureType :type ENetworkFailure%20Enum :default "NetDriverAlreadyExists") (bIsServer :type Boolean))
  (if (not bIsServer)
    (Utilities|DisplayError (CallFunction|NetCodeErrortoString FailureType))))

(event EventHandleTravelError
  (params (FailureType :type ETravelFailure%20Enum :default "NoLevel"))
  (Utilities|DisplayError (CallFunction|TravelErrortoString FailureType)))

(fn HideWidget
  (params (widg :type Widget%20Object%20Reference))
  (Widget|RemovefromParent widg))

(fn NetCodeErrortoString
  (params (inError :type ENetworkFailure%20Enum))
  (switch Utilities|FlowControl|Switch|SwitchonENetworkFailure inError
    (:NetDriverAlreadyExists
      _)
    (:NetDriverCreateFailure
      _)
    (:NetDriverListenFailure
      _)
    (:ConnectionLost
      _)
    (:ConnectionTimeout
      (return "Error: Connection Time Out"))
    (:FailureReceived
      _)
    (:OutdatedClient
      _)
    (:OutdatedServer
      _)
    (:PendingConnectionFailure
      _))
  (return "Error: Lost connection to host"))

(fn TravelErrortoString
  (params (inError :type ETravelFailure%20Enum))
  (return (Utilities|String|Append "Error travelling maps due to" (Utilities|String|EnumtoString inError))))

(fn BeginPlayShowMainMenu
  (if (Utilities|Enum|Equal(Enum) (Variables|Default|GetCurrent%20State) "NewEnumerator0")
    (CallFunction|ShowMainMenu)))

(fn StartPlayingState
  (Utilities|StateTransition "NewEnumerator2"))