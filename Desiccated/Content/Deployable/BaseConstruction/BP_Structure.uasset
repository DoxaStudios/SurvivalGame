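; Deployable base-construction structure that shows a placement preview until it is placed.
; While unplaced, Tick reapplies the able-to-place material, creates a new dynamic instance each frame to tint it translucent green, and zeroes the actor's pitch.
; The replicated Placed flag's OnRep swaps in the final material, enables query and physics collision, and turns off owner-only visibility.
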(event EventTick
  (params (DeltaSeconds :type Float%20%28single-precision%29))
  (bind _returnvalue (Transformation|GetActorRotation))
  (bind _struct (Variables|Default|GetStruct))
  (bind (_roll _pitch _yaw) (Math|Rotator|BreakRotator _returnvalue))
  (if (not (Variables|Default|GetPlaced))
    (Rendering|Material|SetMaterial (Variables|Default|GetStruct) 0 "/Game/Deployable/BaseConstruction/Materials/MI_Able_To_Place.MI_Able_To_Place")
    (bind _returnvalue_2 (Rendering|Material|CreateDynamicMaterialInstance _struct 0 (Rendering|Material|GetMaterial _struct 0) :!class /Script/Engine.PrimitiveComponent))
    (Rendering|Material|SetVectorParameterValue _returnvalue_2 "MyColor" "(R=0.065775,G=1.000000,B=0.000000,A=0.500000)" :!class /Script/Engine.MaterialInstanceDynamic)
    (Transformation|SetActorRotation (Math|Rotator|MakeRotator _roll 0.0 _yaw))))

(fn ConstructionScript)

(fn OnRepPlaced
  (bind _struct (Variables|Default|GetStruct))
  (Rendering|Material|SetMaterial (Variables|Default|GetStruct) 0 (Variables|Default|GetFinal%20Material))
  (Collision|SetCollisionEnabled _struct "QueryAndPhysics")
  (Rendering|SetOnlyOwnerSee _struct false :!class /Script/Engine.PrimitiveComponent))